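; Electric field volume for an electromagnetism lecture that visualizes the field of overlapping BP_Charge actors and completes missions outside lecture mode.
; Overlap registers charges and toggles their physics; on clients, Tick assigns each a pairwise Coulomb force.
; Clients also spawn BP_ElectricPoint tracers that follow the summed inverse-square field, with particle scale and color driven by it.
; Points leaving the volume respawn near random positive charges, or randomly inside if none exist.
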(event `self.ReceiveBeginPlay`
  (`/Engine/EditorBlueprintResources/ActorMacros.Switch Has Authority`
    (:`Remote`
      ;[1 1 1] Spawn Electric Points
      (for _ (range 101)
        (bind _returnvalue (`AddComponent|NODE_AddChildActorComponent-0`))
        (`ChildActorComponent.SetChildActorClass` _returnvalue "/Game/Lecture/ElectricMagnetic/EM01/Blueprint/BP_ElectricPoint.BP_ElectricPoint_C")
        (bind _loc (`self.GetSpawnPoint`))
        (`SceneComponent.K2_SetWorldTransform` _returnvalue (`KismetMathLibrary.MakeTransform` _loc (struct) (`KismetMathLibrary.Conv_DoubleToVector` (`self.scaleValue`))) false false)
        (`SceneComponent.K2_SetWorldTransform` (`Actor.RootComponent` (`ChildActorComponent.ChildActor` _returnvalue)) (`KismetMathLibrary.MakeTransform` _loc (struct) (`KismetMathLibrary.Conv_DoubleToVector` (`self.scaleValue`))) false false)
        (bind _asbp_electric_point (cast `/Game/Lecture/ElectricMagnetic/EM01/Blueprint/BP_ElectricPoint` (`ChildActorComponent.ChildActor` _returnvalue)))
        (`KismetArrayLibrary.Array_Add` (`self.points`) _asbp_electric_point)))))

(event `self.ReceiveTick`
  (params (DeltaSeconds :type "Float (single-precision)"))
  (`/Engine/EditorBlueprintResources/ActorMacros.Switch Has Authority`
    (:`Remote`
      (if (`KismetArrayLibrary.Array_IsValidIndex` (`self.charges`))
        ;[1 1 1] 전기장 내 전하들이 받는 힘 계산
        (for _array_element (`self.charges`)
          (bind _force (`self.GetCoulombForce` _array_element))
          (set `/Game/Lecture/ElectricMagnetic/EM01/Blueprint/BP_Charge.electricForce` _force _array_element))
        ;[1 1 1] 전기장 입자 업데이트
        (for _array_element_2 (`self.points`)
          (bind (_force_2 _color) (`self.GetFieldDirectionOnPos` (`self.GetTransform` _array_element_2)))
          (if (not (`KismetMathLibrary.Vector_IsZero` _force_2))
            (`self.K2_SetActorRotation` _array_element_2 (`KismetMathLibrary.Quat_Rotator` (`KismetMathLibrary.Conv_VectorToQuaternion` _force_2)) false)
            (`SceneComponent.K2_AddWorldOffset` (`Actor.RootComponent` _array_element_2) (* (* (`self.GetActorForwardVector` _array_element_2) DeltaSeconds) (* 5.0 (`self.scaleValue`))) false false)
            (bind _particlesystem (`/Game/Lecture/ElectricMagnetic/EM01/Blueprint/BP_ElectricPoint.ParticleSystem` _array_element_2))
            ;[1 1 1] 전기장 입자 파티클 파라미터 적용 (Size/Color)
            (`FXSystemComponent.SetVectorParameter` _particlesystem "Scale" (`KismetMathLibrary.Conv_DoubleToVector` (`KismetMathLibrary.MapRangeClamped` (`KismetMathLibrary.VSize` _force_2) 20.0 500.0 0.0 1.0)))
            (`FXSystemComponent.SetVectorParameter` _particlesystem "Colorr" (`KismetMathLibrary.Conv_DoubleToVector` (`KismetMathLibrary.MapRangeClamped` _color -200.0 200.0 0.0 1.0)))))))))

(event `Respawn`
  (params (point :type "/Game/Lecture/ElectricMagnetic/EM01/Blueprint/BP_ElectricPoint Object Reference"))
  (bind _particlesystem (`/Game/Lecture/ElectricMagnetic/EM01/Blueprint/BP_ElectricPoint.ParticleSystem` point))
  ;[1 1 1] respawn
  (bind _loc (`self.GetSpawnPoint`))
  (`ParticleSystemComponent.EndTrails` _particlesystem)
  (`self.K2_SetActorLocation` point _loc false false)
  (`ParticleSystemComponent.BeginTrails` _particlesystem "None" "None" "ETrailWidthMode_FromCentre" 0.0))

(event `self.StaticMesh.OnComponentBeginOverlap`
  (params (OverlappedComponent :type "PrimitiveComponent Object Reference") (OtherActor :type "Actor Object Reference") (OtherComp :type "PrimitiveComponent Object Reference") (OtherBodyIndex :type Integer) (bFromSweep :type Boolean) (SweepResult :type "HitResult Structure (by ref)"))
  (bind _gs_base (`/Game/Platform/System/BPFL_SystemLib.GetBaseGameState`))
  (bind _asbp_charge (cast `/Game/Lecture/ElectricMagnetic/EM01/Blueprint/BP_Charge` OtherActor))
  (`|ExecutionSequence`
    (:`then_0`
      (`KismetArrayLibrary.Array_Add` (`self.charges`) _asbp_charge)
      (if (and (`/Game/Lecture/ElectricMagnetic/EM01/Blueprint/BP_Charge.isAffectingElectricField` _asbp_charge) (> (`/Game/Lecture/ElectricMagnetic/EM01/Blueprint/BP_Charge.quantity` _asbp_charge) 0.0))
        (`KismetArrayLibrary.Array_Add` (`self.positiveCharges`) _asbp_charge))
      (set `/Game/Lecture/ElectricMagnetic/EM01/Blueprint/BP_Charge.inElectricField` true _asbp_charge)
      (set `/Game/Lecture/ElectricMagnetic/EM01/Blueprint/BP_Charge.electricField` self _asbp_charge)
      (if (not (`/Game/Lecture/ElectricMagnetic/EM01/Blueprint/BP_Charge.isGripped` _asbp_charge))
        (`PrimitiveComponent.SetSimulatePhysics` (`/Game/Lecture/ElectricMagnetic/EM01/Blueprint/BP_Charge.StaticMesh` _asbp_charge) false)))
    (:`then_1`
      (if (`self.IsLectureMode`)
        _
        (elif (`/Game/Lecture/ElectricMagnetic/EM01/Blueprint/BP_Charge.isAffectingElectricField` _asbp_charge)
          (`/Game/Platform/System/GameState/GS_Base.Complete Mission` _gs_base "Mission00")
          (else
            (`/Game/Platform/System/GameState/GS_Base.Complete Mission` _gs_base "Mission02")))))))

(event `self.StaticMesh.OnComponentEndOverlap`
  (params (OverlappedComponent :type "PrimitiveComponent Object Reference") (OtherActor :type "Actor Object Reference") (OtherComp :type "PrimitiveComponent Object Reference") (OtherBodyIndex :type Integer))
  (`|ExecutionSequence`
    (:`then_0`
      (bind _asbp_charge (cast `/Game/Lecture/ElectricMagnetic/EM01/Blueprint/BP_Charge` OtherActor))
      (if (and (`/Game/Lecture/ElectricMagnetic/EM01/Blueprint/BP_Charge.isAffectingElectricField` _asbp_charge) (> (`/Game/Lecture/ElectricMagnetic/EM01/Blueprint/BP_Charge.quantity` _asbp_charge) 0.0))
        (`KismetArrayLibrary.Array_RemoveItem` (`self.positiveCharges`) _asbp_charge))
      (`KismetArrayLibrary.Array_RemoveItem` (`self.charges`) _asbp_charge)
      (set `/Game/Lecture/ElectricMagnetic/EM01/Blueprint/BP_Charge.inElectricField` false _asbp_charge)
      (if (not (`/Game/Lecture/ElectricMagnetic/EM01/Blueprint/BP_Charge.isGripped` _asbp_charge))
        (`PrimitiveComponent.SetSimulatePhysics` (`/Game/Lecture/ElectricMagnetic/EM01/Blueprint/BP_Charge.StaticMesh` _asbp_charge) true)))
    (:`then_1`
      (bind _asbp_electric_point (cast `/Game/Lecture/ElectricMagnetic/EM01/Blueprint/BP_ElectricPoint` OtherActor))
      (`self.Respawn` _asbp_electric_point))))

(fn `GetCoulombForce`
  (params (charge :type "/Game/Lecture/ElectricMagnetic/EM01/Blueprint/BP_Charge Object Reference"))
  (returns (force :type "Vector Structure"))
  (locals (v :type "Vector Structure"))
  (for _array_element (`self.charges`)
    (if (`/Game/Lecture/ElectricMagnetic/EM01/Blueprint/BP_Charge.isAffectingElectricField` _array_element)
      (bind _returnvalue (- (`SceneComponent.K2_GetComponentLocation` (`Actor.RootComponent` charge)) (`SceneComponent.K2_GetComponentLocation` (`Actor.RootComponent` _array_element))))
      (bind _returnvalue_2 (`KismetMathLibrary.MultiplyMultiply_FloatFloat` (/ (`KismetMathLibrary.VSize` _returnvalue) 100.0) 2.0))
      (set `local.v` (+ (`local.v`) (/ (* (`KismetMathLibrary.Normal` _returnvalue 0.0) (* (`/Game/Lecture/ElectricMagnetic/EM01/Blueprint/BP_Charge.quantity` _array_element) (`/Game/Lecture/ElectricMagnetic/EM01/Blueprint/BP_Charge.quantity` charge))) (select `bool` (== _returnvalue_2 0.0) :`false` _returnvalue_2 :`true` 0.01))))))
  (return (`local.v`)))

(fn `GetFieldDirectionOnPos`
  (params (pos :type "Transform Structure"))
  (returns (force :type "Vector Structure") (Color :type "Float (double-precision)"))
  (locals (v :type "Vector Structure") (f :type "Float (double-precision)"))
  (for _array_element (`self.charges`)
    (if (`/Game/Lecture/ElectricMagnetic/EM01/Blueprint/BP_Charge.isAffectingElectricField` _array_element)
      (bind _returnvalue_location (`KismetMathLibrary.BreakTransform` (`self.GetTransform` _array_element)))
      (bind _returnvalue (- pos_Location _returnvalue_location))
      (bind _quantity (`/Game/Lecture/ElectricMagnetic/EM01/Blueprint/BP_Charge.quantity` _array_element))
      (bind _returnvalue_2 (* (/ (`KismetMathLibrary.VSize` _returnvalue) (`self.scaleValue`)) 0.01))
      (bind _returnvalue_3 (`KismetMathLibrary.MultiplyMultiply_FloatFloat` (select `bool` (< _returnvalue_2 0.01) :`false` _returnvalue_2 :`true` 0.01) 2.0))
      (bind _returnvalue_4 (/ (* (`KismetMathLibrary.Normal` _returnvalue 0.0) (* _quantity (* (`self.scaleValue`) 0.2))) (select `bool` (== _returnvalue_3 0.0) :`false` _returnvalue_3 :`true` 0.01)))
      (set `local.v` (+ _returnvalue_4 (`local.v`)))
      (set `local.f` (+ (* (`KismetMathLibrary.VSize` _returnvalue_4) _quantity) (`local.f`))) ; 전기장 입자 색상
    ))
  (if (`KismetMathLibrary.Vector_IsNearlyZero` (`local.v`) 0.001)
    (return (0.0 0.0 0.0) 0.0)
    (else
      (return (`local.v`) (`local.f`)))))

(fn `GetSpawnPoint`
  (returns (loc :type "Vector Structure"))
  (locals (pos :type "Vector Structure"))
  (bind (_returnvalue_roll _returnvalue_pitch _returnvalue_yaw) (`KismetMathLibrary.BreakRotator` (`self.K2_GetActorRotation`)))
  (bind (_returnvalue_roll_2 _returnvalue_pitch_2 _returnvalue_yaw_2) (`KismetMathLibrary.BreakRotator` (`self.K2_GetActorRotation`)))
  (bind (_returnvalue_roll_3 _returnvalue_pitch_3 _returnvalue_yaw_3) (`KismetMathLibrary.BreakRotator` (`self.K2_GetActorRotation`)))
  (bind _positivecharges (`self.positiveCharges`))
  (bind _output (`|GetArrayItem` _positivecharges (`KismetMathLibrary.RandomIntegerInRange` 0 (- (`KismetArrayLibrary.Array_Length` _positivecharges) 1))))
  (if (> (`KismetArrayLibrary.Array_Length` (`self.positiveCharges`)) 0)
    (return (+ (`KismetMathLibrary.RotateAngleAxis` (`KismetMathLibrary.Vector_BoundedToCube` (`KismetMathLibrary.RotateAngleAxis` (+ (- (`SceneComponent.K2_GetComponentLocation` (`/Game/Lecture/ElectricMagnetic/EM01/Blueprint/BP_Charge.StaticMesh` _output)) (`SceneComponent.K2_GetComponentLocation` (`self.Scene`))) (`KismetMathLibrary.RandomPointInBoundingBox` (0.0 0.0 0.0) (`KismetMathLibrary.Conv_DoubleToVector` (* (`/Game/Lecture/ElectricMagnetic/EM01/Blueprint/BP_Charge.scaleValue` _output) 50.0)))) (* _returnvalue_yaw -1.0) (`self.GetActorUpVector`)) (`self.extent`)) _returnvalue_yaw_3 (`self.GetActorUpVector`)) (`SceneComponent.K2_GetComponentLocation` (`self.Scene`))))
    (else
      (return (+ (`KismetMathLibrary.RotateAngleAxis` (`KismetMathLibrary.RandomPointInBoundingBox` (0.0 0.0 0.0) (`KismetMathLibrary.Conv_DoubleToVector` (- (`self.extent`) 1.0))) _returnvalue_yaw_2 (`self.GetActorUpVector`)) (`SceneComponent.K2_GetComponentLocation` (`self.Scene`)))))))

(fn `UserConstructionScript`
  (locals (NewLocalVar_0 :type "Array of Object Object Reference"))
  ;[1 1 1] 자기장 Volume 설정
  (`SceneComponent.SetRelativeScale3D` (`self.StaticMesh`) (`KismetMathLibrary.Conv_DoubleToVector` (* (`self.extent`) 0.00215))))