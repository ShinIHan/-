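; Grippable point-charge actor for an electromagnetism lecture, scaled as a sphere whose volume follows charge magnitude and colored red or blue by sign.
; While ungripped and affected by an electric field, it moves by a swept, speed-clamped offset from ElectricForce, ticking during physics to follow the field's update.
; Release enables physics only outside the field, and overlapping a BP_ElectricPoint asks the field to respawn that point.
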(event `self.ReceiveBeginPlay`
  (`/Game/Platform/System/BPFL_SystemLib.Init Dynamic Material Instance` (`self.StaticMesh`))
  (`self.SetTickGroup` "TG_DuringPhysics") ; electricField의 tick 이후에 charge의 tick이 실행되도록 설정
  (`self.UpdateChargeColor`))

(event `self.ReceiveTick`
  (params (DeltaSeconds :type "Float (single-precision)"))
  ;[1 1 1] 전하 이동 갱신
  (`|ExecutionSequence`
    (:`then_0`
      (if (and (`self.isAffectedByElectricField`) (`self.inElectricField`) (not (`self.isGripped`)))
        (`self.K2_AddActorWorldOffset` (* (`KismetMathLibrary.ClampVectorSize` (* (`self.electricForce`) (`self.speedValue`)) 0.0 (`self.maxSpeed`)) DeltaSeconds) true)))))

(event `GripInterface.OnGrip`
  (params (GripComponent :type "GripComponent Object Reference") (GripInformation :type "GripInformation Structure (by ref)"))
  ;[1 1 1] Pickup and Drop Event
  (set `self.isGripped` true))

(event `GripInterface.OnGripRelease`
  (params (ReleasingGripComponent :type "GripComponent Object Reference") (GripInformation :type "GripInformation Structure (by ref)"))
  (bind _staticmesh (`self.StaticMesh`))
  ;[1 1 1] Pickup and Drop Event
  (set `self.isGripped` false)
  (if (`self.inElectricField`)
    (`PrimitiveComponent.SetSimulatePhysics` _staticmesh false)
    (else
      (`PrimitiveComponent.SetSimulatePhysics` _staticmesh true))))

(event `self.StaticMesh.OnComponentBeginOverlap`
  (params (OverlappedComponent :type "PrimitiveComponent Object Reference") (OtherActor :type "Actor Object Reference") (OtherComp :type "PrimitiveComponent Object Reference") (OtherBodyIndex :type Integer) (bFromSweep :type Boolean) (SweepResult :type "HitResult Structure (by ref)"))
  (bind _asbp_electric_point (cast `/Game/Lecture/ElectricMagnetic/EM01/Blueprint/BP_ElectricPoint` OtherActor))
  (`/Game/Lecture/ElectricMagnetic/EM01/Blueprint/BP_ElectricField.Respawn` (`self.electricField`) _asbp_electric_point))

(fn `AnimateDissolve`
  (params (deltaTime :type "Float (double-precision)")))

(fn `bDenyGrip`
  (params (GripComponent :type "GripComponent Object Reference"))
  (returns (ReturnValue :type Boolean))
  (return false))

(fn `bDenyHighlight`
  (params (GripComponent :type "GripComponent Object Reference"))
  (returns (ReturnValue :type Boolean))
  (return false))

(fn `bDropSimulate`
  (returns (ReturnValue :type Boolean))
  (return false))

(fn `GetGripRepMoveType`
  (returns (ReturnValue :type "EGripRepMoveType Enum"))
  (return "Client_CompAttach"))

(fn `GetGripType`
  (returns (ReturnValue :type "EGripType Enum"))
  (return "NoPhysicsGrip"))

(fn `GetRadiusFromQuantity`
  (params (volume :type "Float (double-precision)"))
  (returns (radius :type "Float (double-precision)"))
  (return (* (`KismetMathLibrary.MultiplyMultiply_FloatFloat` (/ (* (`KismetMathLibrary.Abs` volume) 0.75) 3.141592) 0.333333) (`self.scaleValue`))))

(fn `IsHeld`
  (returns (HoldingComponents :type "Array of GripComponent Object Reference") (isHeld :type Boolean))
  (return _ false))

(fn `SetDissolveParameterOnMaterial`
  (params (value :type "Float (double-precision)")))

(fn `UpdateChargeColor`
  (locals (MID_Charge :type "MaterialInstanceDynamic Object Reference"))
  (bind _mid_charge (`local.MID_Charge`))
  (bind _returnvalue (>= (`self.quantity`) 0.0))
  (bind `_as머티리얼_인스턴스_다이내믹` (cast `MaterialInstanceDynamic` (`PrimitiveComponent.GetMaterial` (`self.StaticMesh`) 0)))
  (set `local.MID_Charge` `_as머티리얼_인스턴스_다이내믹`)
  (`|ExecutionSequence`
    (:`then_0`
      (`MaterialInstanceDynamic.SetVectorParameterValue` _mid_charge "BaseColor" (select `bool` _returnvalue :`false` (struct :`B` 1.0 :`A` 1.0) :`true` (struct :`R` 1.0 :`A` 1.0) :!type "LinearColor Structure"))
      (`MaterialInstanceDynamic.SetVectorParameterValue` _mid_charge "DissolveEmissiveColor" (select `bool` _returnvalue :`false` (struct :`B` 50.0 :`A` 1.0) :`true` (struct :`R` 50.0 :`A` 1.0) :!type "LinearColor Structure")))
    (:`then_1`
      (if (`self.isAffectingElectricField`)
        (`MaterialInstanceDynamic.SetVectorParameterValue` (`local.MID_Charge`) "Emissive Color" (select `bool` (>= (`self.quantity`) 0.0) :`false` (struct :`B` 50.0 :`A` 1.0) :`true` (struct :`R` 50.0 :`A` 1.0) :!type "LinearColor Structure"))
        (else
          (`MaterialInstanceDynamic.SetVectorParameterValue` :`self` (`local.MID_Charge`) :`ParameterName` "Emissive Color"))))))

(fn `UserConstructionScript`
  (bind _radius (`self.GetRadiusFromQuantity` (`self.quantity`)))
  (`self.SetActorScale3D` (`KismetMathLibrary.Conv_DoubleToVector` _radius)))