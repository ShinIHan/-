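; BP_VoltageDetector is a probe for an electromagnetism lecture that displays the voltage inside an electric field.
; Its sphere overlap stores the BP_ElectricField and completes Mission03 on entry, then clears the reference on exit.
; Tick samples the field's force at the sphere and shows its scaled magnitude in volts on a WBP_Voltage widget.
; Runtime logic runs only without authority; distance-based text scaling is left unconnected.
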(event `self.ReceiveTick`
  (params (DeltaSeconds :type "Float (single-precision)"))
  (`/Engine/EditorBlueprintResources/ActorMacros.Switch Has Authority`
    (:`Remote`
      (`|ExecutionSequence`
        (:`then_0`
          ;[1 1 1] Update electricForce
          (if (`KismetSystemLibrary.IsValid` (`self.electricField`))
            (bind _force (`/Game/Lecture/ElectricMagnetic/EM01/Blueprint/BP_ElectricField.GetFieldDirectionOnPos` (`self.electricField`) (`SceneComponent.K2_GetComponentToWorld` (`self.Sphere`))))
            (bind _output_get (set `self.electricForce` _force))))
        (:`then_1`
          ;[1 1 1] Update voltageText
          (bind _aswbp_voltage (cast `/Game/Lecture/ElectricMagnetic/EM01/Blueprint/WBP_Voltage` (`WidgetComponent.GetUserWidgetObject` (`self.Widget`))))
          (`/Game/Lecture/ElectricMagnetic/EM01/Blueprint/WBP_Voltage.SetVoltageText` _aswbp_voltage (`KismetTextLibrary.Conv_StringToText` (`KismetStringLibrary.Concat_StrStr` (`KismetTextLibrary.Conv_TextToString` (`KismetTextLibrary.Conv_DoubleToText` (* (`KismetMathLibrary.VSize` (`self.electricForce`)) 0.02) "HalfToEven" false true 1 324 0 2)) " V"))))))))

(event `self.Sphere.OnComponentBeginOverlap`
  (params (OverlappedComponent :type "PrimitiveComponent Object Reference") (OtherActor :type "Actor Object Reference") (OtherComp :type "PrimitiveComponent Object Reference") (OtherBodyIndex :type Integer) (bFromSweep :type Boolean) (SweepResult :type "HitResult Structure (by ref)"))
  (`/Engine/EditorBlueprintResources/ActorMacros.Switch Has Authority`
    (:`Remote`
      (bind _asbp_electric_field (cast `/Game/Lecture/ElectricMagnetic/EM01/Blueprint/BP_ElectricField` OtherActor))
      (set `self.electricField` _asbp_electric_field)
      (`/Game/Platform/System/GameState/GS_Base.Complete Mission` (`/Game/Platform/System/BPFL_SystemLib.GetBaseGameState`) "Mission03"))))

(event `self.Sphere.OnComponentEndOverlap`
  (params (OverlappedComponent :type "PrimitiveComponent Object Reference") (OtherActor :type "Actor Object Reference") (OtherComp :type "PrimitiveComponent Object Reference") (OtherBodyIndex :type Integer))
  (`/Engine/EditorBlueprintResources/ActorMacros.Switch Has Authority`
    (:`Remote`
      (cast `/Game/Lecture/ElectricMagnetic/EM01/Blueprint/BP_ElectricField` OtherActor)
      (set `self.electricField` null))))

(fn `UserConstructionScript`
  (bind (_onecolormaterial _twocolormaterial) (`/Game/Platform/System/BPFL_SystemLib.Create Outline Material` (`self.Body`)))
  (set `self.One Color Material` _onecolormaterial)
  (set `self.Two Color Material` _twocolormaterial))