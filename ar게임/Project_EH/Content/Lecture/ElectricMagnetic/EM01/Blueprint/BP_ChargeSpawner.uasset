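; BP_ChargeSpawner is a slider-controlled dispenser that spawns BP_Charge actors in an electric-field lesson, only on the Remote authority branch.
; It spawns a charge after BeginPlay and another whenever the current one leaves its sphere.
; The slider sets signed quantity, kept at least one in magnitude, updating charge size, color and red/blue body emissive.
; Affecting decides whether charges create or receive the field; negative settings on affecting spawners complete Mission01.
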(event `self.ReceiveBeginPlay`
  (`KismetSystemLibrary.Delay` 1.0)
  (`self.SpawnCharge`)
  (`self.SetSliderColor`))

(event `self.Slider.SliderPercentageChanged`
  (params (Alpha :type "Float (double-precision)"))
  (bind _charge (`self.charge`))
  (bind _returnvalue (- (* Alpha 20.0) 10.0))
  (bind _returnvalue_2 (`KismetMathLibrary.Abs` _returnvalue))
  ;[1 1 1] Set Charge Quantity To Slider Progress Point
  (`/Engine/EditorBlueprintResources/ActorMacros.Switch Has Authority`
    (:`Remote`
      (if (not (== Alpha 0.5))
        (if (< Alpha 0.5)
          ;;[1 1 1] Mission
          (if (`self.Affecting`)
            (`/Game/Platform/System/GameState/GS_Base.Complete Mission` (`/Game/Platform/System/BPFL_SystemLib.GetBaseGameState`) "Mission01")))
        (bind _output_get (set `/Game/Lecture/ElectricMagnetic/EM01/Blueprint/BP_Charge.quantity` (select `bool` (< _returnvalue_2 1.0) :`false` _returnvalue :`true` (/ _returnvalue _returnvalue_2)) _charge))
        (set `self.sliderQuantity` _output_get)
        (bind _radius (`/Game/Lecture/ElectricMagnetic/EM01/Blueprint/BP_Charge.GetRadiusFromQuantity` _charge _output_get))
        (`SceneComponent.SetWorldScale3D` (`/Game/Lecture/ElectricMagnetic/EM01/Blueprint/BP_Charge.StaticMesh` _charge) (`KismetMathLibrary.Conv_DoubleToVector` _radius))
        (`/Game/Lecture/ElectricMagnetic/EM01/Blueprint/BP_Charge.UpdateChargeColor` _charge)
        (`self.SetSliderColor`)))))

(event `self.SphereCollision.OnComponentEndOverlap`
  (params (OverlappedComponent :type "PrimitiveComponent Object Reference") (OtherActor :type "Actor Object Reference") (OtherComp :type "PrimitiveComponent Object Reference") (OtherBodyIndex :type Integer))
  (if (== OtherActor (`self.charge`))
    (`self.SpawnCharge`)))

(fn `SetSliderColor`
  (bind _spawnerbody (`self.SpawnerBody`))
  (if (> (`self.sliderQuantity`) 0.0)
    (`MeshComponent.SetVectorParameterValueOnMaterials` _spawnerbody "Emissive" (`KismetMathLibrary.MakeVector` (* (`self.sliderQuantity`) 5.0)))
    (else
      (`MeshComponent.SetVectorParameterValueOnMaterials` _spawnerbody "Emissive" (`KismetMathLibrary.MakeVector` 0.0 0.0 (`KismetMathLibrary.Abs` (* (`self.sliderQuantity`) 5.0)))))))

(fn `SpawnCharge`
  (`/Engine/EditorBlueprintResources/ActorMacros.Switch Has Authority`
    (:`Remote`
      (bind _returnvalue (`|SpawnActorFromClass` "/Game/Lecture/ElectricMagnetic/EM01/Blueprint/BP_Charge.BP_Charge_C" (`SceneComponent.K2_GetComponentToWorld` (`self.SphereCollision`)) "Undefined" "OverrideRootScale" null (`self.sliderQuantity`) (not (`self.Affecting`)) (`self.Affecting`) null))
      (`/Engine/EditorBlueprintResources/StandardMacros.IsValid` _returnvalue
        (:`Is Valid`
          (set `self.charge` _returnvalue))))))

(fn `UserConstructionScript`
  (bind (_onecolormaterial _twocolormaterial) (`/Game/Platform/System/BPFL_SystemLib.Create Outline Material` (`self.SpawnerBody`)))
  (set `self.One Color Material` _onecolormaterial)
  (set `self.Two Color Material` _twocolormaterial))