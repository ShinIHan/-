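; BP_HammerAndNail is an animated Work and Energy lecture prop showing a hammer swinging while hammer and nail heat up in color.
; BeginPlay creates dynamic material instances for both meshes, and SetAnimate toggles the animation.
; While animating, Tick advances two wrapped timers through SetT: one pitches the hammer with an absolute sine, the other lerps both materials from normal to heated color, snapping back each cycle.
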(event `self.ReceiveBeginPlay`
  (bind _returnvalue (`PrimitiveComponent.CreateDynamicMaterialInstance` (`self.SM_Nail`) 0 "/Game/Lecture/WorkAndEnergy/Material/MI_IronBall.MI_IronBall" "BaseColor"))
  (set `self.DynamicNailMateral` _returnvalue)
  (bind _returnvalue_2 (`PrimitiveComponent.CreateDynamicMaterialInstance` (`self.SM_Hammer`) 0 "/Game/Lecture/WorkAndEnergy/Material/MI_IronBall.MI_IronBall" "BaseColor"))
  (set `self.DynamicHammerMateral` _returnvalue_2))

(event `self.ReceiveTick`
  (params (DeltaSeconds :type "Float (single-precision)"))
  (bind _returnvalue (`KismetMathLibrary.LinearColorLerp` (`self.NormalColor`) (`self.HeatedColor`) (`self.MatT`)))
  (if (`self.Animate`)
    (`self.SetT` DeltaSeconds)
    (`SceneComponent.K2_SetRelativeRotation` (`self.SM_Hammer`) (`KismetMathLibrary.MakeRotator` 0.0 (* (`KismetMathLibrary.Abs` (`KismetMathLibrary.Sin` (* (`self.PosT`) 2.5))) 55.0)) false false)
    (`MaterialInstanceDynamic.SetVectorParameterValue` (`self.DynamicNailMateral`) "BaseColor" _returnvalue)
    (`MaterialInstanceDynamic.SetVectorParameterValue` (`self.DynamicHammerMateral`) "BaseColor" _returnvalue)))

(event `SetAnimate`
  (params (NewAnimate :type Boolean))
  (set `self.Animate` NewAnimate))

(fn `SetT`
  (params (DeltaT :type "Float (double-precision)"))
  (set `self.MatT` (mod (+ (* DeltaT 0.2) (`self.MatT`)) 1.0))
  (set `self.PosT` (mod (+ DeltaT (`self.PosT`)) (* 3.141592 2.0))))

(fn `UserConstructionScript`)