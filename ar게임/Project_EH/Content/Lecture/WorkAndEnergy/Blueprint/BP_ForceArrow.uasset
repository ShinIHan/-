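; BP_ForceArrow is a force arrow actor for the Work and Energy lecture, with an optional text label and bobbing animation.
; While animation is on, Tick moves the actor out from its BeginPlay location along the arrow mesh's up vector using an absolute sine bounce.
; SetText updates and shows the label, and SetAnimate toggles the motion.
; Reset hides the label and clears animation state without restoring the actor's location.
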(event `self.ReceiveBeginPlay`
  (set `self.InitialPos` (`self.K2_GetActorLocation`)))

(event `self.ReceiveTick`
  (params (DeltaSeconds :type "Float (single-precision)"))
  (if (`self.ShowAnimation`)
    (bind _output_get (set `self.AnimateT` (+ DeltaSeconds (`self.AnimateT`))))
    (`self.K2_SetActorLocation` (+ (`self.InitialPos`) (* (`SceneComponent.GetUpVector` (`self.SM_ForceArrow`)) (`KismetMathLibrary.Abs` (* (`KismetMathLibrary.Sin` _output_get) 100.0)))))))

(event `SetText`
  (params (NewText :type Text))
  (bind _textrender (`self.TextRender`))
  (`TextRenderComponent.K2_SetText` _textrender NewText)
  (`SceneComponent.SetVisibility` _textrender true false))

(event `Reset`
  (`SceneComponent.SetVisibility` (`self.TextRender`) false false)
  (set `self.ShowAnimation` false)
  (set `self.AnimateT` 0.0))

(event `SetAnimate`
  (params (Value :type Boolean))
  (set `self.ShowAnimation` Value))

(fn `UserConstructionScript`)