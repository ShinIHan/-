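; Ping-pong ball actor for the Work and Energy lecture that loops a grow-and-reset animation on its flattened-ball mesh.
; BeginPlay derives a per-second growth rate from FlattenSpeed, which acts as the growth duration in seconds.
; Tick scales the mesh uniformly up to full size, then a short Delay holds it there before snapping it back to one-tenth scale.
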(event `self.ReceiveBeginPlay`
  (set `self.Span` (/ 0.9 (`self.FlattenSpeed`))))

(event `self.ReceiveTick`
  (params (DeltaSeconds :type "Float (single-precision)"))
  (bind _sm_flattenedball (`self.SM_FlattenedBall`))
  (bind _relativescale3d_x (`KismetMathLibrary.BreakVector` (`SceneComponent.RelativeScale3D` _sm_flattenedball)))
  (bind _returnvalue (+ (* DeltaSeconds (`self.Span`)) _relativescale3d_x))
  (if (<= _relativescale3d_x 1.0)
    (`SceneComponent.SetRelativeScale3D` _sm_flattenedball (`KismetMathLibrary.MakeVector` _returnvalue _returnvalue _returnvalue))
    (else
      (`SceneComponent.SetRelativeScale3D` _sm_flattenedball (1.0 1.0 1.0))
      (`KismetSystemLibrary.Delay` 0.3)
      (`SceneComponent.SetRelativeScale3D` _sm_flattenedball (0.1 0.1 0.1)))))

(fn `UserConstructionScript`)