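; BP_HeatHand is a Work and Energy lecture visual of two hands rubbing back and forth while their color shifts from normal to heated.
; BeginPlay gives each hand mesh a dynamic material instance from MI_NormalHand.
; While SetAnimate has enabled animation, Tick slides the hands in opposite directions on a sine wave and lerps BaseColor.
; SetT advances both timers with wrapping, so the heating restarts from the normal color every five seconds.
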(event `self.ReceiveBeginPlay`
  (bind _returnvalue (`PrimitiveComponent.CreateDynamicMaterialInstance` (`self.Hand_1`) 1 "/Game/Lecture/WorkAndEnergy/Material/MI_NormalHand.MI_NormalHand" "BaseColor"))
  (set `self.DynamicMaterial_1` _returnvalue)
  (bind _returnvalue_2 (`PrimitiveComponent.CreateDynamicMaterialInstance` (`self.Hand_2`) 1 "/Game/Lecture/WorkAndEnergy/Material/MI_NormalHand.MI_NormalHand" "BaseColor"))
  (set `self.DynamicMaterial_2` _returnvalue_2))

(event `self.ReceiveTick`
  (params (DeltaSeconds :type "Float (single-precision)"))
  (bind _returnvalue (`KismetMathLibrary.LinearColorLerp` (`self.NormalHandColor`) (`self.HeatedHandColor`) (`self.MatT`)))
  (bind _returnvalue_2 (`KismetMathLibrary.Sin` (* (`self.PosT`) 5.0)))
  (if (`self.Animate`)
    (`self.SetT` DeltaSeconds)
    (`SceneComponent.K2_SetRelativeLocation` (`self.Hand_1`) (`KismetMathLibrary.MakeVector` (* _returnvalue_2 -20.0) -10.0) false false)
    (`SceneComponent.K2_SetRelativeLocation` (`self.Hand_2`) (`KismetMathLibrary.MakeVector` (* _returnvalue_2 20.0) 10.0) false false)
    (`MaterialInstanceDynamic.SetVectorParameterValue` (`self.DynamicMaterial_1`) "BaseColor" _returnvalue)
    (`MaterialInstanceDynamic.SetVectorParameterValue` (`self.DynamicMaterial_2`) "BaseColor" _returnvalue)))

(event `SetAnimate`
  (params (NewAnimate :type Boolean))
  (set `self.Animate` NewAnimate))

(fn `SetT`
  (params (DeltaT :type "Float (double-precision)"))
  (set `self.MatT` (mod (+ (* DeltaT 0.2) (`self.MatT`)) 1.0))
  (set `self.PosT` (mod (+ DeltaT (`self.PosT`)) (* 3.141592 2.0))))

(fn `UserConstructionScript`)