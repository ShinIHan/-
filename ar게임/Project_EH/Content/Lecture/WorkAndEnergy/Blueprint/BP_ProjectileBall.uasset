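; Projectile ball for the Work and Energy lecture, flying under manually integrated gravity.
; Shoot derives speed from the kinetic energy relation sqrt(2·Force/Mass), treating Force as energy, converts to centimetres and launches along the actor's local -Y.
; Tick moves it without sweep until it falls below LimitZ; overlapping a BP_ProjectileMove also destroys it.
; On destruction it calls ShootBall on its BP_ProjectileMove reference, triggering another shot.
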(event `self.ReceiveBeginPlay`)

(event `self.ReceiveTick`
  (params (DeltaSeconds :type "Float (single-precision)"))
  (bind (_returnvalue_x _returnvalue_y _returnvalue_z) (`KismetMathLibrary.BreakVector` (`self.K2_GetActorLocation`)))
  (if (`self.Simulate`)
    (bind _output_get (set `self.Velocity` (+ (`self.Velocity`) (`KismetMathLibrary.MakeVector` 0.0 0.0 (* -980.0 DeltaSeconds)))))
    (`self.K2_SetActorLocation` (+ (`self.K2_GetActorLocation`) (* _output_get (`KismetMathLibrary.MakeVector` DeltaSeconds DeltaSeconds DeltaSeconds))))
    (if (< _returnvalue_z (`self.LimitZ`))
      (`self.K2_DestroyActor`))))

(event `Shoot`
  (params (Mass :type "Float (double-precision)") (Force :type "Float (double-precision)") (LimitZ :type "Float (double-precision)") (Ref :type "/Game/Lecture/WorkAndEnergy/Blueprint/BP_ProjectileMove Object Reference"))
  (bind _output_get (set `self.Mass` Mass))
  (set `self.LimitZ` LimitZ)
  (set `self.Ref` Ref)
  (set `self.Velocity` (`KismetMathLibrary.GreaterGreater_VectorRotator` (* (* (`KismetMathLibrary.Sqrt` (`KismetMathLibrary.Abs` (* Force (/ 2.0 _output_get)))) 100.0) (0.0 -1.0 0.0)) (`self.K2_GetActorRotation`)))
  (set `self.Simulate` true))

(event `self.ReceiveDestroyed`
  (bind _asbp_projectile_move (cast `/Game/Lecture/WorkAndEnergy/Blueprint/BP_ProjectileMove` (`self.Ref`)))
  (`/Game/Lecture/WorkAndEnergy/Blueprint/BP_ProjectileMove.ShootBall` _asbp_projectile_move))

(event `self.StaticMesh.OnComponentBeginOverlap`
  (params (OverlappedComponent :type "PrimitiveComponent Object Reference") (OtherActor :type "Actor Object Reference") (OtherComp :type "PrimitiveComponent Object Reference") (OtherBodyIndex :type Integer) (bFromSweep :type Boolean) (SweepResult :type "HitResult Structure (by ref)"))
  (cast `/Game/Lecture/WorkAndEnergy/Blueprint/BP_ProjectileMove` OtherActor)
  (`self.K2_DestroyActor`))

(fn `UserConstructionScript`)