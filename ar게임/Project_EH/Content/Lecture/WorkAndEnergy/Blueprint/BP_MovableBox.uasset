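; Movable box for a work-and-energy physics lecture that slides and slows to a stop under simulated friction.
; AddForce stores a friction coefficient and sets velocity per axis as sqrt(2·Force/Mass), scaled by 100, treating Force like kinetic energy.
; Tick moves the box manually without sweep and applies friction deceleration from a normal force of mass times gravity, clamping to zero.
; Reset clears velocity and restores the starting location.
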(event `self.ReceiveBeginPlay`
  (set `self.DefaultPos` (`self.K2_GetActorLocation`))
  (set `self.NormalForce` (* (`self.Mass`) 980.0)))

(event `self.ReceiveTick`
  (params (DeltaSeconds :type "Float (single-precision)"))
  (bind _velocity (`self.Velocity`))
  (bind _returnvalue (* (* (`KismetMathLibrary.Normal` _velocity) -1.0) (* (/ (* (`self.NormalForce`) (`self.FrictionCoefficient`)) (`self.Mass`)) DeltaSeconds)))
  (`self.K2_SetActorLocation` (+ (`self.K2_GetActorLocation`) (* _velocity (`KismetMathLibrary.MakeVector` DeltaSeconds DeltaSeconds DeltaSeconds))))
  (if (<= (`KismetMathLibrary.VSize` _velocity) (`KismetMathLibrary.VSize` _returnvalue))
    (set `self.Velocity` (0.0 0.0 0.0))
    (else
      (set `self.Velocity` (+ _velocity _returnvalue)))))

(event `AddForce`
  (params (Force :type "Vector Structure") (FrictionCoefficient :type "Float (double-precision)"))
  (bind _returnvalue (/ 2.0 (`self.Mass`)))
  (set `self.Velocity` (`KismetMathLibrary.MakeVector` (* (`KismetMathLibrary.Sqrt` (* Force_X _returnvalue)) 100.0) (* (`KismetMathLibrary.Sqrt` (* Force_Y _returnvalue)) 100.0) (* (`KismetMathLibrary.Sqrt` (* Force_Z _returnvalue)) 100.0)))
  (set `self.FrictionCoefficient` FrictionCoefficient))

(event `Reset`
  (set `self.Velocity` (0.0 0.0 0.0))
  (`self.K2_SetActorLocation` (`self.DefaultPos`)))

(fn `UserConstructionScript`)