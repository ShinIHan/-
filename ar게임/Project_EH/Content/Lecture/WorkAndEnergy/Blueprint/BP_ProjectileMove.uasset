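; Projectile launcher for a work and energy lecture, firing a ball and visualizing its kinetic, potential and mechanical energy.
; Plus/minus buttons adjust mass, force and barrel angle, update monitors, and complete missions at target values.
; ShootBall spawns BP_ProjectileBall after a delay and passes it those launch settings.
; Tick derives energies from ball speed and height above the launcher, scaling bars relative to the total.
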(event `self.ReceiveTick`
  (params (DeltaSeconds :type "Float (single-precision)"))
  (if (`KismetSystemLibrary.IsValid` (`self.ProjectileBall`))
    (bind _output_get (`self.SetKeneticEnergy`))
    (bind _output_get_2 (`self.SetPotentialEnergy`))
    (set `self.Energy_Mechanical` (+ _output_get _output_get_2))
    (`SceneComponent.SetRelativeScale3D` (`self.MechanicalEnergy`) (1.0 1.0 0.5))
    (`SceneComponent.SetRelativeScale3D` (`self.KeneticEnergy`) (`KismetMathLibrary.MakeVector` 1.0 1.0 (* (/ (`self.Energy_Kenetic`) (`self.Energy_Mechanical`)) 0.5)))
    (`SceneComponent.SetRelativeScale3D` (`self.PotentialEnergy`) (`KismetMathLibrary.MakeVector` 1.0 1.0 (* (/ (`self.Energy_Potential`) (`self.Energy_Mechanical`)) 0.5)))))

(event `ShootBall`
  (bind _firelocation (`self.FireLocation`))
  (bind (_returnvalue_x _returnvalue_y _returnvalue_z) (`KismetMathLibrary.BreakVector` (`SceneComponent.K2_GetComponentLocation` (`self.SM_ProjectileBody`))))
  (`KismetSystemLibrary.Delay` 1.0)
  (bind _returnvalue (`|SpawnActorFromClass` "/Game/Lecture/WorkAndEnergy/Blueprint/BP_ProjectileBall.BP_ProjectileBall_C" (`KismetMathLibrary.MakeTransform` (`SceneComponent.K2_GetComponentLocation` _firelocation) (`SceneComponent.K2_GetComponentRotation` _firelocation) (0.1 0.1 0.1)) "Undefined" "MultiplyWithRoot" null null))
  (bind _output_get (set `self.ProjectileBall` _returnvalue))
  (`/Game/Lecture/WorkAndEnergy/Blueprint/BP_ProjectileBall.Shoot` _output_get (`self.Mass`) (`self.Force`) _returnvalue_z self))

(event `self.RedPlusButton.ButtonStateChanged`
  (params (State :type Boolean))
  (bind _returnvalue (+ (`self.Mass`) 1.0))
  (set `self.RedPlusPressed` (not (`self.RedPlusPressed`)))
  (`/Game/Platform/VRSystem/InteractionObject/Component/ButtonComponent.SetLastTogglePressTime` (`self.RedPlusButton`))
  (if (`self.RedPlusPressed`)
    (if (<= _returnvalue 15.0)
      (bind _output_get (set `self.Mass` _returnvalue))
      (`TextRenderComponent.K2_SetText` (`self.RedMonitorText`) (`KismetTextLibrary.Conv_StringToText` (`KismetStringLibrary.Concat_StrStr` (`KismetStringLibrary.Conv_IntToString` (`KismetMathLibrary.FTrunc` _output_get)) "kg")))
      (if (== (`self.Mass`) 8.0)
        (`/Game/Platform/System/GameState/GS_Base.Complete Mission` (`/Game/Platform/System/BPFL_SystemLib.GetBaseGameState`) "Mission00")))))

(event `self.RedMinusButton.ButtonStateChanged`
  (params (State :type Boolean))
  (bind _returnvalue (- (`self.Mass`) 1.0))
  (set `self.RedMinusPressed` (not (`self.RedMinusPressed`)))
  (`/Game/Platform/VRSystem/InteractionObject/Component/ButtonComponent.SetLastTogglePressTime` (`self.RedMinusButton`))
  (if (`self.RedMinusPressed`)
    (if (> _returnvalue 0.0)
      (bind _output_get (set `self.Mass` _returnvalue))
      (`TextRenderComponent.K2_SetText` (`self.RedMonitorText`) (`KismetTextLibrary.Conv_StringToText` (`KismetStringLibrary.Concat_StrStr` (`KismetStringLibrary.Conv_IntToString` (`KismetMathLibrary.FTrunc` _output_get)) "kg")))
      (if (== (`self.Mass`) 8.0)
        (`/Game/Platform/System/GameState/GS_Base.Complete Mission` (`/Game/Platform/System/BPFL_SystemLib.GetBaseGameState`) "Mission00")))))

(event `self.BluePlusButton.ButtonStateChanged`
  (params (State :type Boolean))
  (bind _returnvalue (+ (`self.Force`) 10.0))
  (set `self.BluePlusPressed` (not (`self.BluePlusPressed`)))
  (`/Game/Platform/VRSystem/InteractionObject/Component/ButtonComponent.SetLastTogglePressTime` (`self.BluePlusButton`))
  (if (`self.BluePlusPressed`)
    (if (<= _returnvalue 300.0)
      (bind _output_get (set `self.Force` _returnvalue))
      (`TextRenderComponent.K2_SetText` (`self.BlueMonitorText`) (`KismetTextLibrary.Conv_StringToText` (`KismetStringLibrary.Concat_StrStr` (`KismetStringLibrary.Conv_IntToString` (`KismetMathLibrary.FTrunc` _output_get)) "N")))
      (if (== (`self.Force`) 40.0)
        (`/Game/Platform/System/GameState/GS_Base.Complete Mission` (`/Game/Platform/System/BPFL_SystemLib.GetBaseGameState`) "Mission01")))))

(event `self.BlueMinusButton.ButtonStateChanged`
  (params (State :type Boolean))
  (bind _returnvalue (- (`self.Force`) 10.0))
  (set `self.BlueMinusPressed` (not (`self.BlueMinusPressed`)))
  (`/Game/Platform/VRSystem/InteractionObject/Component/ButtonComponent.SetLastTogglePressTime` (`self.BlueMinusButton`))
  (if (`self.BlueMinusPressed`)
    (if (>= _returnvalue 20.0)
      (bind _output_get (set `self.Force` _returnvalue))
      (`TextRenderComponent.K2_SetText` (`self.BlueMonitorText`) (`KismetTextLibrary.Conv_StringToText` (`KismetStringLibrary.Concat_StrStr` (`KismetStringLibrary.Conv_IntToString` (`KismetMathLibrary.FTrunc` _output_get)) "N")))
      (if (== (`self.Force`) 40.0)
        (`/Game/Platform/System/GameState/GS_Base.Complete Mission` (`/Game/Platform/System/BPFL_SystemLib.GetBaseGameState`) "Mission01")))))

(event `self.YellowPlusButton.ButtonStateChanged`
  (params (State :type Boolean))
  (bind _returnvalue (+ (`self.Degree`) 5.0))
  (set `self.YellowPlusPressed` (not (`self.YellowPlusPressed`)))
  (`/Game/Platform/VRSystem/InteractionObject/Component/ButtonComponent.SetLastTogglePressTime` (`self.YellowPlusButton`))
  (if (`self.YellowPlusPressed`)
    (if (< _returnvalue 90.0)
      (bind _output_get (set `self.Degree` _returnvalue))
      (`SceneComponent.K2_SetRelativeRotation` (`self.SM_ProjectileBarrel`) (`KismetMathLibrary.MakeRotator` _output_get) false false)
      (`TextRenderComponent.K2_SetText` (`self.YellowMonitorText`) (`KismetTextLibrary.Conv_StringToText` (`KismetStringLibrary.Concat_StrStr` (`KismetStringLibrary.Conv_IntToString` (`KismetMathLibrary.FTrunc` _output_get)) "°")))
      (if (== (`self.Degree`) 45.0)
        (`/Game/Platform/System/GameState/GS_Base.Complete Mission` (`/Game/Platform/System/BPFL_SystemLib.GetBaseGameState`) "Mission02")))))

(event `self.YellowMinusButton.ButtonStateChanged`
  (params (State :type Boolean))
  (bind _returnvalue (- (`self.Degree`) 5.0))
  (set `self.YellowMinusPressed` (not (`self.YellowMinusPressed`)))
  (`/Game/Platform/VRSystem/InteractionObject/Component/ButtonComponent.SetLastTogglePressTime` (`self.YellowMinusButton`))
  (if (`self.YellowMinusPressed`)
    (if (>= _returnvalue 0.0)
      (bind _output_get (set `self.Degree` _returnvalue))
      (`SceneComponent.K2_SetRelativeRotation` (`self.SM_ProjectileBarrel`) (`KismetMathLibrary.MakeRotator` _output_get) false false)
      (`TextRenderComponent.K2_SetText` (`self.YellowMonitorText`) (`KismetTextLibrary.Conv_StringToText` (`KismetStringLibrary.Concat_StrStr` (`KismetStringLibrary.Conv_IntToString` (`KismetMathLibrary.FTrunc` _output_get)) "°")))
      (if (== (`self.Degree`) 45.0)
        (`/Game/Platform/System/GameState/GS_Base.Complete Mission` (`/Game/Platform/System/BPFL_SystemLib.GetBaseGameState`) "Mission02")))))

(fn `SetKeneticEnergy`
  (returns (Output_Get :type "Float (double-precision)"))
  (bind _output_get (set `self.Energy_Kenetic` (* (`KismetMathLibrary.MultiplyMultiply_FloatFloat` (`KismetMathLibrary.VSize` (* (`/Game/Lecture/WorkAndEnergy/Blueprint/BP_ProjectileBall.Velocity` (`self.ProjectileBall`)) (0.01 0.01 0.01))) 2.0) (* (`self.Mass`) 0.5))))
  (return _output_get))

(fn `SetPotentialEnergy`
  (returns (Output_Get :type "Float (double-precision)"))
  (bind (_returnvalue_x _returnvalue_y _returnvalue_z) (`KismetMathLibrary.BreakVector` (`SceneComponent.K2_GetComponentLocation` (`self.SM_ProjectileBody`))))
  (bind (_returnvalue_x_2 _returnvalue_y_2 _returnvalue_z_2) (`KismetMathLibrary.BreakVector` (`self.K2_GetActorLocation` (`self.ProjectileBall`))))
  (bind _output_get (set `self.Energy_Potential` (* (* (`self.Mass`) 9.8) (* (- _returnvalue_z_2 _returnvalue_z) 0.01))))
  (return _output_get))

(fn `UserConstructionScript`)