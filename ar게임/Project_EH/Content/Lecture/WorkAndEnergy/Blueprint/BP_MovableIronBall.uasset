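; BP_MovableIronBall is an iron ball actor for a work and energy lecture that falls under hand-coded gravity.
; While simulation is on, Tick integrates a constant downward acceleration into velocity and moves the actor without sweep, so collisions do not stop it.
; SimulateBall starts the motion, and Reset clears velocity, returns the ball to the position saved at BeginPlay and stops simulation.
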(event `self.ReceiveBeginPlay`
  (set `self.DefaultPos` (`self.K2_GetActorLocation`)))

(event `self.ReceiveTick`
  (params (DeltaSeconds :type "Float (single-precision)"))
  (if (`self.Simulate`)
    (bind _output_get (set `self.Velocity` (+ (`self.Velocity`) (`KismetMathLibrary.MakeVector` 0.0 0.0 (* -980.0 DeltaSeconds)))))
    (`self.K2_SetActorLocation` (+ (`self.K2_GetActorLocation`) (* _output_get (`KismetMathLibrary.MakeVector` DeltaSeconds DeltaSeconds DeltaSeconds))))))

(event `SimulateBall`
  (set `self.Simulate` true))

(event `Reset`
  (set `self.Velocity` (0.0 0.0 0.0))
  (`self.K2_SetActorLocation` (`self.DefaultPos`))
  (set `self.Simulate` false))

(fn `UserConstructionScript`)