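; BP_Pendulum is an actor in the work and energy lecture content that swings a rope mesh as an idealized pendulum.
; BeginPlay derives the period from RopeLength with the small-angle formula 2π√(L/g).
; Each Tick advances elapsed time wrapped by that period, then sets SMRope's world roll to MaxAngle times a cosine of it, a closed-form motion without physics simulation.
; CheckMoreThanMaxAngle is an unused stub.
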(event `self.ReceiveBeginPlay`
  (`self.SetCycle`)
  (set `self.TimeElapsed` 0.0))

(event `self.ReceiveTick`
  (params (DeltaSeconds :type "Float (single-precision)"))
  (bind _output_get (`self.SetTimeElapsed` DeltaSeconds))
  (`self.SetAngle` _output_get))

(fn `CheckMoreThanMaxAngle`
  (params (NewAngle :type "Float (double-precision)")))

(fn `SetAngle`
  (params (A :type "Float (double-precision)"))
  (`SceneComponent.K2_SetWorldRotation` (`self.SM_Rope`) (`KismetMathLibrary.MakeRotator` (* (`self.MaxAngle`) (`KismetMathLibrary.Cos` (* A (/ 6.283184 (`self.Cycle`)))))) false false))

(fn `SetCycle`
  (set `self.Cycle` (* 6.283184 (`KismetMathLibrary.Sqrt` (/ (`self.RopeLength`) 9.81)))))

(fn `SetTimeElapsed`
  (params (A :type "Float (double-precision)"))
  (returns (Output_Get :type "Float (double-precision)"))
  (bind _output_get (set `self.TimeElapsed` (mod (+ A (`self.TimeElapsed`)) (`self.Cycle`))))
  (return _output_get))

(fn `UserConstructionScript`)