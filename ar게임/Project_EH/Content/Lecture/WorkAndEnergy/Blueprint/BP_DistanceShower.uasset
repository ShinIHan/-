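; BP_DistanceShower is a distance indicator actor for the Work and Energy lecture, pairing a text label with a static mesh.
; SetActive writes the supplied text to the TextRender and shows it, while Reset only hides that label, leaving the mesh untouched.
; SetScale places the mesh at the actor's location and rotation, stretching its Y scale to the distance divided by 100.
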(event `SetActive`
  (params (NewText :type Text))
  (bind _textrender (`self.TextRender`))
  (`TextRenderComponent.K2_SetText` _textrender NewText)
  (`SceneComponent.SetVisibility` _textrender true false))

(event `Reset`
  (`SceneComponent.SetVisibility` (`self.TextRender`) false false))

(event `SetScale`
  (params (Distance :type "Float (double-precision)"))
  (`SceneComponent.K2_SetWorldTransform` (`self.Static Mesh`) (`KismetMathLibrary.MakeTransform` (`self.K2_GetActorLocation`) (`self.K2_GetActorRotation`) (`KismetMathLibrary.MakeVector` 1.0 (/ Distance 100.0) 1.0)) false false))

(fn `UserConstructionScript`)