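; VR finger pointer actor that lets the player interact with widget components by laser or touch.
; While active, Tick line-traces forward, feeds hits to WidgetInteraction and sizes the ray and end-point marker.
; ActiveWidget activates it or relays pointer press/release, restarting a timeline that drives material alpha, then deactivates it.
; Touch clicks fire when EndPoint stops overlapping a widget, provided a short forward trace still hits that widget.
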(event `self.ReceiveTick`
  (params (DeltaSeconds :type "Float (single-precision)"))
  (bind _returnvalue (`self.K2_GetActorLocation`))
  (bind _ray (`self.Ray`))
  (bind _endpoint (`self.EndPoint`))
  (bind _relativescale3d_x (`KismetMathLibrary.BreakVector` (`SceneComponent.RelativeScale3D` _endpoint)))
  (if (`self.IsLineTraceActive`)
    (bind _asbp_vrcharacter (cast `/Game/Platform/Character/Base/BP_VRCharacter` (`GameplayStatics.GetPlayerCharacter` 0)))
    (bind (_outhit _returnvalue_2) (`KismetSystemLibrary.LineTraceSingle` _returnvalue (+ _returnvalue (* (`self.GetActorForwardVector`) (`WidgetInteractionComponent.InteractionDistance` (`self.WidgetInteraction`)))) "TraceTypeQuery1" false (`self.MakeIgnoreActorArray` _asbp_vrcharacter) "None" true (struct :`G` 0.02957 :`B` 1.0 :`A` 1.0) (struct :`R` 1.0 :`B` 0.031819 :`A` 1.0)))
    (bind _output_get (set `self.Out Hit` _outhit))
    (if _returnvalue_2
      (bind _returnvalue_3 (* (`.Time` (`GameplayStatics.BreakHitResult` _output_get)) (`WidgetInteractionComponent.InteractionDistance` (`self.WidgetInteraction`))))
      (bind _returnvalue_4 (`KismetMathLibrary.MakeVector` _returnvalue_3 1.0 1.0))
      (`SceneComponent.SetWorldScale3D` _ray _returnvalue_4)
      (`WidgetInteractionComponent.SetCustomHitResult` (`self.WidgetInteraction`) (`self.Out Hit`))
      (`SceneComponent.K2_SetRelativeLocation` _endpoint (`KismetMathLibrary.MakeVector` (+ _returnvalue_3 (* _relativescale3d_x 2.0))) false false)
      (`SceneComponent.SetHiddenInGame` _endpoint false false)
      (else
        (`SceneComponent.SetWorldScale3D` _ray _returnvalue_4)
        (`SceneComponent.SetHiddenInGame` _endpoint true false)))))

(event `ResetDeactiveTimeline`
  (bind (_direction _deactivealpha) (`Timeline|DeactiveTimeline` :!via `PlayFromStart`)
    (:`Update`
      (`MaterialInstanceDynamic.SetScalarParameterValue` (`self.MI_Spline`) "Alpha" _deactivealpha)
      (`MaterialInstanceDynamic.SetScalarParameterValue` (`self.MI_EndPoint`) "Alpha" _deactivealpha))
    (:`Finished`
      (`self.SetActivation` false))))

(event `self.EndPoint.OnComponentBeginOverlap`
  (params (OverlappedComponent :type "PrimitiveComponent Object Reference") (OtherActor :type "Actor Object Reference") (OtherComp :type "PrimitiveComponent Object Reference") (OtherBodyIndex :type Integer) (bFromSweep :type Boolean) (SweepResult :type "HitResult Structure (by ref)"))
  ;[1 1 1] End Point Overlap
  (bind `_as위젯_컴포넌트` (cast `WidgetComponent` OtherComp))
  (set `self.BeginOverlappedWidgetComponent` `_as위젯_컴포넌트`))

(event `self.EndPoint.OnComponentEndOverlap`
  (params (OverlappedComponent :type "PrimitiveComponent Object Reference") (OtherActor :type "Actor Object Reference") (OtherComp :type "PrimitiveComponent Object Reference") (OtherBodyIndex :type Integer))
  ;[1 1 1] End Point Overlap
  (bind `_as위젯_컴포넌트` (cast `WidgetComponent` OtherComp))
  (if (and (== (`self.GetLastHitComponent`) `_as위젯_컴포넌트`) (== `_as위젯_컴포넌트` (`self.BeginOverlappedWidgetComponent`)))
    (bind _hitcomponent (`self.EndPointLineTrace` (`self.EndPoint`)))
    (if (== _hitcomponent (`self.BeginOverlappedWidgetComponent`))
      (`self.WidgetInteractionClick` (`self.WidgetInteraction`)))
    (set `self.BeginOverlappedWidgetComponent` null)
    (`WidgetInteractionComponent.SetCustomHitResult` (`self.WidgetInteraction`) (`self.EmptyHitResult`))
    (else
      (set `self.BeginOverlappedWidgetComponent` null)
      (`WidgetInteractionComponent.SetCustomHitResult` (`self.WidgetInteraction`) (`self.EmptyHitResult`)))))

(fn `ActiveWidget`
  (params (Pressed :type Boolean))
  (returns (Success :type Boolean))
  (bind _widgetinteraction (`self.WidgetInteraction`))
  (bind _widgetinteraction_2 (`self.WidgetInteraction`))
  (bind _returnvalue (or (`WidgetInteractionComponent.IsOverInteractableWidget` _widgetinteraction_2) (`WidgetInteractionComponent.IsOverFocusableWidget` _widgetinteraction_2)))
  (if (`self.IsLineTraceActive`)
    (`self.ResetDeactiveTimeline`)
    (if _returnvalue
      (if (`local.Pressed`)
        (`WidgetInteractionComponent.PressPointerKey` _widgetinteraction "LeftMouseButton")
        (else
          (`WidgetInteractionComponent.ReleasePointerKey` _widgetinteraction "LeftMouseButton")))
      (return _returnvalue)
      (else
        _))
    (else
      (`self.SetActivation` true)))
  (return true))

(fn `EndPointLineTrace`
  (params (EndPoint :type "SceneComponent Object Reference"))
  (returns (HitComponent :type "PrimitiveComponent Object Reference"))
  (bind _returnvalue (`SceneComponent.K2_GetComponentLocation` EndPoint))
  (bind (_outhit _returnvalue_2) (`KismetSystemLibrary.LineTraceSingle` _returnvalue (+ _returnvalue (* (`SceneComponent.GetForwardVector` EndPoint) (`self.EndOverlapLineTraceDistance`))) "TraceTypeQuery1")) ; End Overlap시 앞에 같은 Widget Component가 존재하는지 체크하기 위한 Line Trace
  (if _returnvalue_2
    (return (`.HitComponent` (`GameplayStatics.BreakHitResult` _outhit)))))

(fn `GetLastHitComponent`
  (returns (HitComponent :type "PrimitiveComponent Object Reference"))
  (return (`.HitComponent` (`GameplayStatics.BreakHitResult` (`WidgetInteractionComponent.GetLastHitResult` (`self.WidgetInteraction`))))))

(fn `MakeIgnoreActorArray`
  (params (VRCharacter :type "Object Object Reference"))
  (returns (IgonreActorArray :type "Array of Actor Object Reference"))
  (return (`|MakeArray` (`self.GetOwner`))))

(fn `SetActivation`
  (params (IsActivation :type Boolean))
  (bind _output_get (set `self.IsLineTraceActive` IsActivation))
  (`self.SetActorTickEnabled` _output_get)
  (`SceneComponent.SetVisibility` (`self.WidgetInteraction`) _output_get false)
  (`SceneComponent.SetVisibility` (`self.EndPoint`) _output_get false)
  (`SceneComponent.SetVisibility` (`self.Ray`) _output_get false)
  (if IsActivation
    (`self.ResetDeactiveTimeline`)))

(fn `SetFingerWidgetActivation`
  (params (IsActivation :type Boolean))
  (bind _output_get (set `self.IsLineTraceActive` IsActivation))
  (`self.SetActorTickEnabled` _output_get)
  (`SceneComponent.SetVisibility` (`self.WidgetInteraction`) true false)
  (`SceneComponent.SetVisibility` (`self.EndPoint`) true false)
  (`SceneComponent.SetVisibility` (`self.Ray`) true false))

(fn `UserConstructionScript`
  (bind _returnvalue (`PrimitiveComponent.CreateDynamicMaterialInstance` (`self.Ray`) 0 "/Game/Graphic/Teleporter/Material/M_SplineArc.M_SplineArc" "None"))
  (set `self.MI_Spline` _returnvalue)
  (bind _returnvalue_2 (`PrimitiveComponent.CreateDynamicMaterialInstance` (`self.EndPoint`) 0 "/Game/Graphic/Teleporter/Material/M_EndPoint.M_EndPoint" "None"))
  (set `self.MI_EndPoint` _returnvalue_2))

(fn `WidgetInteractionClick`
  (params (WidgetInteraction :type "WidgetInteractionComponent Object Reference"))
  (`WidgetInteractionComponent.PressPointerKey` WidgetInteraction "LeftMouseButton")
  (`WidgetInteractionComponent.ReleasePointerKey` WidgetInteraction "LeftMouseButton"))