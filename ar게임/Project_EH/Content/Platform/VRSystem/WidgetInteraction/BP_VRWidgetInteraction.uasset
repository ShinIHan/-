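; VR laser pointer actor that lets the player press UMG widgets through a WidgetInteraction component.
; While active, Tick line-traces forward, stretches the ray, places the end point on hits and feeds each hit to the component as a custom result.
; ActiveWidgetInteraction wakes an inactive pointer or forwards left-mouse press and release over usable widgets.
; Activation and input restart a timeline that drives material Alpha, then switches the pointer off.
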(event `self.ReceiveTick`
  (params (DeltaSeconds :type "Float (single-precision)"))
  (bind _returnvalue (`self.K2_GetActorLocation`))
  (bind _endpoint (`self.EndPoint`))
  (if (`self.IsLinetraceActive`)
    (bind _asbp_vrcharacter (cast `/Game/Platform/Character/Base/BP_VRCharacter` (`GameplayStatics.GetPlayerCharacter` 0)))
    (bind (_outhit _returnvalue_2) (`KismetSystemLibrary.LineTraceSingle` _returnvalue (+ _returnvalue (* (`self.GetActorForwardVector`) (`self.SplineMaxDistance`))) "TraceTypeQuery1" false (`self.MakeIgnoreActorArray` _asbp_vrcharacter)))
    (bind _output_get (set `self.Out Hit` _outhit))
    (if _returnvalue_2
      (bind _returnvalue_3 (* (`.Time` (`GameplayStatics.BreakHitResult` _output_get)) (`self.SplineMaxDistance`)))
      (bind _returnvalue_4 (`KismetMathLibrary.MakeVector` _returnvalue_3 1.0 1.0))
      (`SceneComponent.SetWorldScale3D` (`self.Ray`) _returnvalue_4)
      (`WidgetInteractionComponent.SetCustomHitResult` (`self.WidgetInteraction`) (`self.Out Hit`))
      (`SceneComponent.K2_SetRelativeLocation` _endpoint (`KismetMathLibrary.MakeVector` _returnvalue_3) false false)
      (`SceneComponent.SetHiddenInGame` _endpoint false false)
      (else
        (`SceneComponent.SetWorldScale3D` (`self.Ray`) _returnvalue_4)
        (`SceneComponent.SetHiddenInGame` _endpoint true false)))))

(event `ResetDeactiveTimeline`
  (bind (_direction _deactivealpha) (`Timeline|DeactiveTimeline` :!via `PlayFromStart`)
    (:`Update`
      (`MaterialInstanceDynamic.SetScalarParameterValue` (`self.MI_Spline`) "Alpha" _deactivealpha)
      (`MaterialInstanceDynamic.SetScalarParameterValue` (`self.MI_EndPoint`) "Alpha" _deactivealpha))
    (:`Finished`
      (`self.SetActivation` false))))

(fn `ActiveWidgetInteraction`
  (params (Pressed :type Boolean))
  (returns (Success :type Boolean))
  (bind _widgetinteraction (`self.WidgetInteraction`))
  (bind _widgetinteraction_2 (`self.WidgetInteraction`))
  (bind _returnvalue (or (`WidgetInteractionComponent.IsOverInteractableWidget` _widgetinteraction_2) (`WidgetInteractionComponent.IsOverFocusableWidget` _widgetinteraction_2)))
  (if (`self.IsLineTraceActive`)
    (`self.ResetDeactiveTimeline`)
    (if _returnvalue
      (if (`local.Pressed`)
        (`WidgetInteractionComponent.PressPointerKey` _widgetinteraction "LeftMouseButton")
        (else
          (`WidgetInteractionComponent.ReleasePointerKey` _widgetinteraction "LeftMouseButton")))
      (return _returnvalue)
      (else
        _))
    (else
      (`self.SetActivation` true)))
  (return true))

(fn `MakeIgnoreActorArray`
  (params (VRCharacter :type "Object Object Reference"))
  (returns (IgonreActorArray :type "Array of Actor Object Reference"))
  (return (`|MakeArray` (`self.GetOwner`))))

(fn `SetActivation`
  (params (IsActivation :type Boolean))
  (bind _output_get (set `self.IsLineTraceActive` IsActivation))
  (`self.SetActorTickEnabled` _output_get)
  (`SceneComponent.SetVisibility` (`self.WidgetInteraction`) _output_get false)
  (`SceneComponent.SetVisibility` (`self.EndPoint`) _output_get false)
  (`SceneComponent.SetVisibility` (`self.Ray`) _output_get false)
  (if IsActivation
    (`self.ResetDeactiveTimeline`)))

(fn `UserConstructionScript`
  (bind _returnvalue (`PrimitiveComponent.CreateDynamicMaterialInstance` (`self.Ray`) 0 "/Game/Graphic/Teleporter/Material/M_SplineArc.M_SplineArc" "None"))
  (set `self.MI_Spline` _returnvalue)
  (bind _returnvalue_2 (`PrimitiveComponent.CreateDynamicMaterialInstance` (`self.EndPoint`) 0 "/Game/Graphic/Teleporter/Material/M_EndPoint.M_EndPoint" "None"))
  (set `self.MI_EndPoint` _returnvalue_2))