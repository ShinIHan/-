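; VR hand auto-posing Blueprint that curls each finger from input and stops it when it touches something.
; Begin and end overlap events on two trigger components per finger record contact in the TriggersOverlap map.
; TrackingInput passes thumb, index and a shared value for the other fingers to SetAllFingerIKCol, which updates only fingers without overlaps.
; ApplyAlpha moves each finger alpha toward GripTarget, floored by input, at a frame-rate-independent GripSpeed.
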(event `self.thumb_01.OnComponentBeginOverlap`
  (params (OverlappedComponent :type "PrimitiveComponent Object Reference") (OtherActor :type "Actor Object Reference") (OtherComp :type "PrimitiveComponent Object Reference") (OtherBodyIndex :type Integer) (bFromSweep :type Boolean) (SweepResult :type "HitResult Structure (by ref)"))
  ;[1 1 1] Thumb
  (`BlueprintMapLibrary.Map_Add` (`self.TriggersOverlap`) "NewEnumerator0" true))

(event `self.middle_01.OnComponentBeginOverlap`
  (params (OverlappedComponent :type "PrimitiveComponent Object Reference") (OtherActor :type "Actor Object Reference") (OtherComp :type "PrimitiveComponent Object Reference") (OtherBodyIndex :type Integer) (bFromSweep :type Boolean) (SweepResult :type "HitResult Structure (by ref)"))
  ;[1 1 1] Middle
  (`BlueprintMapLibrary.Map_Add` (`self.TriggersOverlap`) "NewEnumerator4" true))

(event `self.index_01.OnComponentBeginOverlap`
  (params (OverlappedComponent :type "PrimitiveComponent Object Reference") (OtherActor :type "Actor Object Reference") (OtherComp :type "PrimitiveComponent Object Reference") (OtherBodyIndex :type Integer) (bFromSweep :type Boolean) (SweepResult :type "HitResult Structure (by ref)"))
  ;[1 1 1] Index
  (`BlueprintMapLibrary.Map_Add` (`self.TriggersOverlap`) "NewEnumerator2" true))

(event `self.ring_01.OnComponentBeginOverlap`
  (params (OverlappedComponent :type "PrimitiveComponent Object Reference") (OtherActor :type "Actor Object Reference") (OtherComp :type "PrimitiveComponent Object Reference") (OtherBodyIndex :type Integer) (bFromSweep :type Boolean) (SweepResult :type "HitResult Structure (by ref)"))
  ;[1 1 1] Ring
  (`BlueprintMapLibrary.Map_Add` (`self.TriggersOverlap`) "NewEnumerator6" true))

(event `self.pinky_01.OnComponentBeginOverlap`
  (params (OverlappedComponent :type "PrimitiveComponent Object Reference") (OtherActor :type "Actor Object Reference") (OtherComp :type "PrimitiveComponent Object Reference") (OtherBodyIndex :type Integer) (bFromSweep :type Boolean) (SweepResult :type "HitResult Structure (by ref)"))
  ;[1 1 1] Pinky
  (`BlueprintMapLibrary.Map_Add` (`self.TriggersOverlap`) "NewEnumerator8" true))

(event `self.thumb_01.OnComponentEndOverlap`
  (params (OverlappedComponent :type "PrimitiveComponent Object Reference") (OtherActor :type "Actor Object Reference") (OtherComp :type "PrimitiveComponent Object Reference") (OtherBodyIndex :type Integer))
  ;[1 1 1] Thumb
  (`BlueprintMapLibrary.Map_Add` (`self.TriggersOverlap`) "NewEnumerator0"))

(event `self.index_01.OnComponentEndOverlap`
  (params (OverlappedComponent :type "PrimitiveComponent Object Reference") (OtherActor :type "Actor Object Reference") (OtherComp :type "PrimitiveComponent Object Reference") (OtherBodyIndex :type Integer))
  ;[1 1 1] Index
  (`BlueprintMapLibrary.Map_Add` (`self.TriggersOverlap`) "NewEnumerator2"))

(event `self.ring_01.OnComponentEndOverlap`
  (params (OverlappedComponent :type "PrimitiveComponent Object Reference") (OtherActor :type "Actor Object Reference") (OtherComp :type "PrimitiveComponent Object Reference") (OtherBodyIndex :type Integer))
  ;[1 1 1] Ring
  (`BlueprintMapLibrary.Map_Add` (`self.TriggersOverlap`) "NewEnumerator6"))

(event `self.middle_01.OnComponentEndOverlap`
  (params (OverlappedComponent :type "PrimitiveComponent Object Reference") (OtherActor :type "Actor Object Reference") (OtherComp :type "PrimitiveComponent Object Reference") (OtherBodyIndex :type Integer))
  ;[1 1 1] Middle
  (`BlueprintMapLibrary.Map_Add` (`self.TriggersOverlap`) "NewEnumerator4"))

(event `self.pinky_01.OnComponentEndOverlap`
  (params (OverlappedComponent :type "PrimitiveComponent Object Reference") (OtherActor :type "Actor Object Reference") (OtherComp :type "PrimitiveComponent Object Reference") (OtherBodyIndex :type Integer))
  ;[1 1 1] Pinky
  (`BlueprintMapLibrary.Map_Add` (`self.TriggersOverlap`) "NewEnumerator8"))

(event `self.middle_03.OnComponentBeginOverlap`
  (params (OverlappedComponent :type "PrimitiveComponent Object Reference") (OtherActor :type "Actor Object Reference") (OtherComp :type "PrimitiveComponent Object Reference") (OtherBodyIndex :type Integer) (bFromSweep :type Boolean) (SweepResult :type "HitResult Structure (by ref)"))
  ;[1 1 1] Middle
  (`BlueprintMapLibrary.Map_Add` (`self.TriggersOverlap`) "NewEnumerator5" true))

(event `self.index_03.OnComponentBeginOverlap`
  (params (OverlappedComponent :type "PrimitiveComponent Object Reference") (OtherActor :type "Actor Object Reference") (OtherComp :type "PrimitiveComponent Object Reference") (OtherBodyIndex :type Integer) (bFromSweep :type Boolean) (SweepResult :type "HitResult Structure (by ref)"))
  ;[1 1 1] Index
  (`BlueprintMapLibrary.Map_Add` (`self.TriggersOverlap`) "NewEnumerator3" true))

(event `self.ring_03.OnComponentBeginOverlap`
  (params (OverlappedComponent :type "PrimitiveComponent Object Reference") (OtherActor :type "Actor Object Reference") (OtherComp :type "PrimitiveComponent Object Reference") (OtherBodyIndex :type Integer) (bFromSweep :type Boolean) (SweepResult :type "HitResult Structure (by ref)"))
  ;[1 1 1] Ring
  (`BlueprintMapLibrary.Map_Add` (`self.TriggersOverlap`) "NewEnumerator7" true))

(event `self.pinky_03.OnComponentBeginOverlap`
  (params (OverlappedComponent :type "PrimitiveComponent Object Reference") (OtherActor :type "Actor Object Reference") (OtherComp :type "PrimitiveComponent Object Reference") (OtherBodyIndex :type Integer) (bFromSweep :type Boolean) (SweepResult :type "HitResult Structure (by ref)"))
  ;[1 1 1] Pinky
  (`BlueprintMapLibrary.Map_Add` (`self.TriggersOverlap`) "NewEnumerator9" true))

(event `self.thumb_03.OnComponentBeginOverlap`
  (params (OverlappedComponent :type "PrimitiveComponent Object Reference") (OtherActor :type "Actor Object Reference") (OtherComp :type "PrimitiveComponent Object Reference") (OtherBodyIndex :type Integer) (bFromSweep :type Boolean) (SweepResult :type "HitResult Structure (by ref)"))
  ;[1 1 1] Thumb
  (`BlueprintMapLibrary.Map_Add` (`self.TriggersOverlap`) "NewEnumerator1" true))

(event `self.thumb_03.OnComponentEndOverlap`
  (params (OverlappedComponent :type "PrimitiveComponent Object Reference") (OtherActor :type "Actor Object Reference") (OtherComp :type "PrimitiveComponent Object Reference") (OtherBodyIndex :type Integer))
  ;[1 1 1] Thumb
  (`BlueprintMapLibrary.Map_Add` (`self.TriggersOverlap`) "NewEnumerator1"))

(event `self.index_03.OnComponentEndOverlap`
  (params (OverlappedComponent :type "PrimitiveComponent Object Reference") (OtherActor :type "Actor Object Reference") (OtherComp :type "PrimitiveComponent Object Reference") (OtherBodyIndex :type Integer))
  ;[1 1 1] Index
  (`BlueprintMapLibrary.Map_Add` (`self.TriggersOverlap`) "NewEnumerator3"))

(event `self.ring_03.OnComponentEndOverlap`
  (params (OverlappedComponent :type "PrimitiveComponent Object Reference") (OtherActor :type "Actor Object Reference") (OtherComp :type "PrimitiveComponent Object Reference") (OtherBodyIndex :type Integer))
  ;[1 1 1] Ring
  (`BlueprintMapLibrary.Map_Add` (`self.TriggersOverlap`) "NewEnumerator7"))

(event `self.pinky_03.OnComponentEndOverlap`
  (params (OverlappedComponent :type "PrimitiveComponent Object Reference") (OtherActor :type "Actor Object Reference") (OtherComp :type "PrimitiveComponent Object Reference") (OtherBodyIndex :type Integer))
  ;[1 1 1] Pinky
  (`BlueprintMapLibrary.Map_Add` (`self.TriggersOverlap`) "NewEnumerator9"))

(event `self.middle_03.OnComponentEndOverlap`
  (params (OverlappedComponent :type "PrimitiveComponent Object Reference") (OtherActor :type "Actor Object Reference") (OtherComp :type "PrimitiveComponent Object Reference") (OtherBodyIndex :type Integer))
  ;[1 1 1] Middle
  (`BlueprintMapLibrary.Map_Add` (`self.TriggersOverlap`) "NewEnumerator5"))

(fn `ApplyAlpha`
  (params (Alpha :type "Float (double-precision)") (Finger :type "/Game/Platform/VRSystem/Hand/E_Finger Enum" :default "NewEnumerator0"))
  (bind _returnvalue (* (`self.GripSpeed`) (`GameplayStatics.GetWorldDeltaSeconds`)))
  (bind _returnvalue_2 (select `/Game/Platform/VRSystem/Hand/E_Finger` (`local.Finger`) :`NewEnumerator0` (`self.ThumbAlpha`) :`NewEnumerator1` (`self.IndexAlpha`) :`NewEnumerator2` (`self.MiddleAlpha`) :`NewEnumerator3` (`self.RingAlpha`) :`NewEnumerator4` (`self.PinkyAlpha`)))
  (bind _result (`|EaseFunction` "Linear" (+ (`KismetMathLibrary.FClamp` (- (`KismetMathLibrary.FClamp` (`self.GripTarget`) Alpha) _returnvalue_2) (* _returnvalue -1.0) _returnvalue) _returnvalue_2) 0.0 1.0))
  (switch `/Game/Platform/VRSystem/Hand/E_Finger` Finger
    (:`NewEnumerator0`
      (set `self.ThumbAlpha` _result))
    (:`NewEnumerator1`
      (set `self.IndexAlpha` _result))
    (:`NewEnumerator2`
      (set `self.MiddleAlpha` _result))
    (:`NewEnumerator3`
      (set `self.RingAlpha` _result))
    (:`NewEnumerator4`
      (set `self.PinkyAlpha` _result))))

(fn `CalculateAlpha`
  (params (TraceLength :type "Float (double-precision)") (ArrowNum :type Integer))
  (returns (Ratio :type "Float (double-precision)"))
  (return (+ (* TraceLength 0.25) (* ArrowNum 0.33))))

(fn `SetAllFingerIK_Col`
  (params (ThumbInputAlpha :type "Float (double-precision)") (IndexInputAlpha :type "Float (double-precision)") (MiddleInputAlpha :type "Float (double-precision)") (RingInputAlpha :type "Float (double-precision)") (PinkyInputAlpha :type "Float (double-precision)"))
  (`|ExecutionSequence`
    (:`then_0`
      (if (`KismetMathLibrary.BooleanNOR` (`BlueprintMapLibrary.Map_Find` (`self.TriggersOverlap`) "NewEnumerator0") (`BlueprintMapLibrary.Map_Find` (`self.TriggersOverlap`) "NewEnumerator1"))
        (`self.ApplyAlpha` (`local.ThumbInputAlpha`))))
    (:`then_1`
      (if (`KismetMathLibrary.BooleanNOR` (`BlueprintMapLibrary.Map_Find` (`self.TriggersOverlap`) "NewEnumerator2") (`BlueprintMapLibrary.Map_Find` (`self.TriggersOverlap`) "NewEnumerator3"))
        (`self.ApplyAlpha` (`local.IndexInputAlpha`) "NewEnumerator1")))
    (:`then_2`
      (if (`KismetMathLibrary.BooleanNOR` (`BlueprintMapLibrary.Map_Find` (`self.TriggersOverlap`) "NewEnumerator4") (`BlueprintMapLibrary.Map_Find` (`self.TriggersOverlap`) "NewEnumerator5"))
        (`self.ApplyAlpha` (`local.MiddleInputAlpha`) "NewEnumerator2")))
    (:`then_3`
      (if (`KismetMathLibrary.BooleanNOR` (`BlueprintMapLibrary.Map_Find` (`self.TriggersOverlap`) "NewEnumerator6") (`BlueprintMapLibrary.Map_Find` (`self.TriggersOverlap`) "NewEnumerator7"))
        (`self.ApplyAlpha` (`local.RingInputAlpha`) "NewEnumerator3")))
    (:`then_4`
      (if (`KismetMathLibrary.BooleanNOR` (`BlueprintMapLibrary.Map_Find` (`self.TriggersOverlap`) "NewEnumerator8") (`BlueprintMapLibrary.Map_Find` (`self.TriggersOverlap`) "NewEnumerator9"))
        (`self.ApplyAlpha` (`local.PinkyInputAlpha`) "NewEnumerator4")))))

(fn `TrackingInput`
  (params (Thumb :type "Float (double-precision)") (Index :type "Float (double-precision)") (Other :type "Float (double-precision)"))
  (`self.SetAllFingerIK_Col` Thumb Index Other Other Other))

(fn `UserConstructionScript`)