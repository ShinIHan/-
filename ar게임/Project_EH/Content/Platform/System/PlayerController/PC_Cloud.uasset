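; PC_Cloud is the player controller for the Cloud platform, handling level travel and forwarding character assignment requests to its parent.
; A server travel request checks whether the current level name contains the part of the target name before the first "0".
; On a match the game mode ServerTravels to the level; otherwise the client switches servers through GI_Cloud's TravelSession.
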(event `self.Client_RequestAssignCharacterByOption`
  ;[1 1 1] Character Spawn / Cloud
  (`parent.Client_RequestAssignCharacterByOption`))

(event `self.Server_RequestAssignCharacter`
  (params (Platform :type "/Game/Platform/System/E_Platform Enum" :default "NewEnumerator0") (SeatNum :type Integer))
  ;[1 1 1] Character Spawn / Cloud
  (`parent.Server_RequestAssignCharacter` Platform SeatNum))

(event `self.Server_RequestTravel`
  (params (LevelName :type String))
  ;[1 1 1] Level Travel
  ;;[1 0.5081 0.4782] 가고자 하는 레벨과 현재의 레벨의 문자열을 비교하여 서버를 옮길 지 레벨만 옮길 지 판단
  (bind _returnvalue (`GameplayStatics.GetCurrentLevelName` true))
  (if (< (`KismetStringLibrary.FindSubstring` _returnvalue (`KismetStringLibrary.Split` LevelName "0")) 0)
    (`self.Client_RequestTravelSession` LevelName) ; 클라가 연결된 서버 자체를 변경
    (else
      (`/Game/Platform/System/GameMode/GM_Base.ServerTravel` (`/Game/Platform/System/BPFL_SystemLib.GetBaseGameMode`) LevelName) ; 서버의 레벨을 변경
    )))

(event `Client_RequestTravelSession`
  (params (LevelName :type String))
  ;[1 1 1] Level Travel
  (bind _asgi_cloud (cast `/Game/Platform/System/GameInstance/GI_Cloud` (`/Game/Platform/System/BPFL_SystemLib.GetBaseGameInstance`)))
  (`/Game/Platform/System/GameInstance/GI_Cloud.TravelSession` _asgi_cloud LevelName))

(fn `UserConstructionScript`
  (`parent.UserConstructionScript`))