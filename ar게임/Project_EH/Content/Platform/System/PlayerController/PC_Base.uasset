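; Base player controller for a multiplayer lecture app, creating the lecture management widget on remote clients.
; Server events handle teleporting and forward character assignment by platform to the game mode, and lecture start, skip and sequence speed to the game state.
; Level travel is an empty event for Local and Cloud subclasses to override, also used by world reset.
; Camera fade helpers are included.
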(event `self.ReceiveBeginPlay`
  (`parent.ReceiveBeginPlay`)
  (`self.Create LectureManagement Widget`))

(event `Create LectureManagement Widget`
  ;[1 1 1] Create Lecture Management Widget
  (`/Engine/EditorBlueprintResources/ActorMacros.Switch Has Authority`
    (:`Remote`
      (bind _returnvalue (`|CreateWidget` "/Game/Widget/LectureManagement/WBP_LectureManagement.WBP_LectureManagement_C" self true true))
      (set `self.Lecture Management Widget` _returnvalue))))

(event `self.ReceivePossess`
  (params (PossessedPawn :type "Pawn Object Reference"))
  ;[1 1 1] Possess
  (`parent.ReceivePossess` PossessedPawn))

(event `Server_Teleport`
  (params (Location :type "Vector Structure") (Rotation :type "Rotator Structure"))
  ;[1 1 1] Teleport
  (`self.K2_TeleportTo` :`self` (`self.K2_GetPawn`) :`DestLocation` Location)
  (`self.Client_SetControlRotation` Rotation))

(event `Client_SetControlRotation`
  (params (Rotation :type "Rotator Structure"))
  ;[1 1 1] Teleport
  (`self.SetControlRotation` Rotation))

(event `Client_RequestAssignCharacterByOption`
  ;[1 1 1] Assign Character / Base / Option : Platform
  (`self.Server_RequestAssignCharacter` (`/Game/Platform/System/GameInstance/GI_Base.Platform` (`/Game/Platform/System/BPFL_SystemLib.GetBaseGameInstance`)) -1))

(event `Server_RequestAssignCharacter`
  (params (Platform :type "/Game/Platform/System/E_Platform Enum" :default "NewEnumerator0") (SeatNum :type Integer))
  ;[1 1 1] Assign Character / Base / Option : Platform
  (`/Game/Platform/System/GameMode/GM_Base.Server_AssignCharacter` (`/Game/Platform/System/BPFL_SystemLib.GetBaseGameMode`) Platform SeatNum self))

(event `Server_RequestLectureStart`
  ;[1 1 1] Lecture Management / Travel Level | Cloud에서는 전부 테스트용으로만 사용되고 실제로는 안쓰인다.
  (`/Game/Platform/System/GameState/GS_Base.ProcessFlow` (`/Game/Platform/System/BPFL_SystemLib.GetBaseGameState`) :!label _label))

(event `Server_RequestTravel`
  (params (LevelName :type String) (`Lecture Row Name` :type Name))
  ;[1 1 1] Lecture Management / Travel Level | Cloud에서는 전부 테스트용으로만 사용되고 실제로는 안쓰인다.
  ;;[0.8122 0.8238 1] 레벨 이동방식은 Local과 Cloud가 다르기 때문에 상속 구조 사용
)

(event `Server_RequestLectureSkip`
  ;[1 1 1] Lecture Management / Travel Level | Cloud에서는 전부 테스트용으로만 사용되고 실제로는 안쓰인다.
  (goto _label))

(event `ResetWorld`
  ;[1 1 1] Lecture Management / Travel Level | Cloud에서는 전부 테스트용으로만 사용되고 실제로는 안쓰인다.
  (bind _returnvalue (`GameplayStatics.GetCurrentLevelName` true))
  (`self.Server_RequestTravel` _returnvalue))

(event `Server_Set Sequence Speed`
  (params (Speed :type "Float (double-precision)"))
  ;[1 1 1] Lecture Management / Travel Level | Cloud에서는 전부 테스트용으로만 사용되고 실제로는 안쓰인다.
  (`/Game/Platform/System/GameState/GS_Base.SequenceFunc_PlaySpeed` (`/Game/Platform/System/BPFL_SystemLib.GetBaseGameState`) Speed))

(fn `CameraFadeIn`
  (params (Duration :type "Float (double-precision)"))
  (`PlayerCameraManager.StartCameraFade` :`self` (`self.PlayerCameraManager`) :`FromAlpha` 1.0 :`Duration` Duration))

(fn `CameraFadeOut`
  (params (Duration :type "Float (double-precision)"))
  (`PlayerCameraManager.StartCameraFade` :`self` (`self.PlayerCameraManager`) :`ToAlpha` 1.0 :`Duration` Duration))

(fn `UserConstructionScript`)