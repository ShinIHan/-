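; PC_Local is the local-platform player controller that relays character assignment and level travel requests to the game mode.
; Character assignment sends Platform and SeatNum from the local game instance through a server request to the game mode's ServerAssignCharacter.
; ResetWorld requests travel back to the current level with the stored Lecture row name.
; The travel request calls the game mode's ServerTravel, then writes that Lecture onto GI_Local.
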(event `self.Client_RequestAssignCharacterByOption`
  (bind _gi_local (`/Game/Platform/System/BPFL_SystemLib.GetLocalGameInstance`))
  ;[1 1 1] Assgin Character / Local / Option : Seat Num
  (`self.Server_RequestAssignCharacter` (`/Game/Platform/System/GameInstance/GI_Base.Platform` _gi_local) (`/Game/Platform/System/GameInstance/GI_Local.SeatNum` _gi_local)))

(event `self.ResetWorld`
  (bind _asgi_local (cast `/Game/Platform/System/GameInstance/GI_Local` (`/Game/Platform/System/BPFL_SystemLib.GetBaseGameInstance`)))
  (bind _returnvalue (`GameplayStatics.GetCurrentLevelName` true))
  (`self.Server_RequestTravel` _returnvalue (`/Game/Platform/System/GameInstance/GI_Local.Lecture` _asgi_local)))

(event `self.Server_RequestAssignCharacter`
  (params (Platform :type "/Game/Platform/System/E_Platform Enum" :default "NewEnumerator0") (SeatNum :type Integer))
  ;[1 1 1] Assgin Character / Local / Option : Seat Num
  (`/Game/Platform/System/GameMode/GM_Base.Server_AssignCharacter` (`/Game/Platform/System/BPFL_SystemLib.GetBaseGameMode`) Platform SeatNum self))

(event `self.Server_RequestTravel`
  (params (LevelName :type String) (`Lecture Row Name` :type Name))
  ;[1 1 1] Level Travel
  (`/Game/Platform/System/GameMode/GM_Base.ServerTravel` (`/Game/Platform/System/BPFL_SystemLib.GetBaseGameMode`) LevelName)
  (bind _asgi_local (cast `/Game/Platform/System/GameInstance/GI_Local` (`/Game/Platform/System/BPFL_SystemLib.GetBaseGameInstance`)))
  (set `/Game/Platform/System/GameInstance/GI_Local.Lecture` `Lecture Row Name` _asgi_local))

(fn `UserConstructionScript`
  (`parent.UserConstructionScript`))