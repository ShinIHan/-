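; Game mode for cloud lectures that seats joining players in a classroom and hands lecture flow data to the game state.
; BeginPlay calls lecture loading, then passes LectureData on after a fixed two-second delay.
; ServerAssignCharacter spawns and initializes each character at the seat named by player count, storing that seat on it.
; The data-table lookup, classroom streaming and seat-map filling are disconnected, leaving the Load_LectureLevel event empty.
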(event `self.ReceiveBeginPlay`
  (bind _gs_base (`/Game/Platform/System/BPFL_SystemLib.GetBaseGameState`))
  (`parent.ReceiveBeginPlay`)
  (`self.Load_LectureLevel`) ; 여기서 서버에서 지정해준 강의 로드해오면 됨
  (`KismetSystemLibrary.Delay` 2.0) ; 클라이언트 접속 대기
  (set `self.GameStateRef` _gs_base)
  (`/Game/Platform/System/GameState/GS_Base.Load_FlowData` _gs_base (`self.LectureData`)))

(event `self.Server_AssignCharacter`
  (params (Platform :type "/Game/Platform/System/E_Platform Enum" :default "NewEnumerator0") (PlayerController :type "PlayerController Object Reference"))
  (bind _returnvalue (`self.GetNumPlayers`))
  (bind _seat (`self.Get_SeatReference` _returnvalue))
  (bind (_returnvalue_location _returnvalue_rotation _returnvalue_scale) (`KismetMathLibrary.BreakTransform` (`self.GetTransform` _seat)))
  (bind _character (`self.SpawnCharacter` (`/Game/Platform/System/GameInstance/GI_Base.Platform` (`/Game/Platform/System/BPFL_SystemLib.GetBaseGameInstance`)) (`KismetMathLibrary.MakeTransform` (+ _returnvalue_location (0.0 0.0 50.0)) _returnvalue_rotation _returnvalue_scale) PlayerController))
  (`self.Initialize Cloud Player` PlayerController)
  (bind _asbp_base_character (cast `/Game/Platform/Character/Base/BP_BaseCharacter` _character))
  (set `/Game/Platform/Character/Base/BP_BaseCharacter.Seat Ref` _seat _asbp_base_character))

(event `Load_LectureLevel`)

(fn `Get_SeatReference`
  (params (PlayerIndex :type Integer))
  (returns (Seat :type "/Game/Platform/LectureBase/BP_Seat Object Reference"))
  (bind (_value _returnvalue) (`BlueprintMapLibrary.Map_Find` (`self.Seats`) (`KismetStringLibrary.Concat_StrStr` "BP_Seat" (`KismetStringLibrary.Conv_IntToString` PlayerIndex))))
  (if _returnvalue
    (return _value)
    (else
      (`KismetSystemLibrary.PrintString` "GM_CloudLecture::GetSeatReference - Cannot find BP_Seat" true true (struct :`R` 1.0 :`A` 1.0) 20.0)
      (return null))))

(fn `Get_StreamLevelName`
  (params (Type :type Byte :default 0))
  (returns (Name :type Name))
  (switch `|SwitchEnum` Type
    (:`NewEnumerator0`
      (return "LV_Classroom_I"))
    (:`NewEnumerator1`
      (return "LV_Classroom_L"))
    (:`NewEnumerator2`
      (return "LV_Classroom_P"))))

(fn `UserConstructionScript`
  (`parent.UserConstructionScript`))