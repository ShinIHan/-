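; Game mode for the Cloud platform that sets up dedicated server services and loads player profiles.
; BeginPlay starts the TCP network helper plus AWS authorizer and gateways on dedicated servers.
; After character assignment, it requests player info from DynamoDB by PlayerSub, then applies name, role and customization and logs level access.
; The failure handler re-requests player info without a retry limit; access-record and connection callbacks are empty.
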(event `self.ReceiveBeginPlay`
  (bind _returnvalue (subsystem `AWSSubsystem`))
  (`parent.ReceiveBeginPlay`)
  (if (`KismetSystemLibrary.IsDedicatedServer`)
    (`|ExecutionSequence`
      (:`then_0`
        (`NetworkTCPSubsystem.StartNetworkHelper` (subsystem `NetworkTCPSubsystem`) (`KismetStringLibrary.Conv_IntToString` (`/Game/Platform/System/GameInstance/GI_Cloud.ServerAcceptabelMaxPlayers` (`/Game/Platform/System/BPFL_SystemLib.GetCloudGameInstance`))) (`|CreateDelegate` :!event `IOCPConnectSuccess`) (`|CreateDelegate` :!event `IOCPConnectFailure`))
        (`AWSSubsystem.StartAuthorizer` _returnvalue)
        (`AWSSubsystem.StartGateways` _returnvalue))
      (:`then_1`))))

(event `self.Server_AssignCharacter`
  (params (Platform :type "/Game/Platform/System/E_Platform Enum" :default "NewEnumerator0") (SeatNum :type Integer) (PlayerController :type "PlayerController Object Reference"))
  ;[1 1 1] Character Spawn / Cloud
  (`parent.Server_AssignCharacter` Platform 0 PlayerController)
  (`/Engine/EditorBlueprintResources/StandardMacros.IsValid` PlayerController
    (:`Is Valid`
      (`self.Initialize Cloud Player` PlayerController) ; Lecture에서도 쓰여서 함수로 묶음
    )))

(fn `AddAccessRecordFailure`
  (params (FailureReason :type String)))

(fn `AddAccessRecordSuccess`)

(fn `GetNow`
  (returns (Now :type "DateTime Structure"))
  (locals (IsTest :type Boolean))
  (bind _returnvalue (`KismetMathLibrary.Now`))
  (bind _returnvalue_2 (- (`KismetMathLibrary.Now`) (`KismetMathLibrary.UtcNow`)))
  (return (select `bool` (`local.IsTest`) :`false` (select `bool` (or (> (`KismetMathLibrary.MakeTimespan` 0 -1) _returnvalue_2) (> _returnvalue_2 (`KismetMathLibrary.MakeTimespan` 0 1))) :`false` (+ _returnvalue (`KismetMathLibrary.MakeTimespan` 0 9)) :`true` _returnvalue) :`true` (`KismetMathLibrary.MakeDateTime` 2022 11 25 15 57))))

(fn `GetPlayerInfoFaulure`
  (params (RequestResult :type String) (PlayerSub :type String))
  (bind _returnvalue (`AWSSubsystem.GetDynamoDBGateway` (subsystem `AWSSubsystem`)))
  (`/Engine/EditorBlueprintResources/StandardMacros.IsValid` _returnvalue
    (:`Is Valid`
      (`DynamoDBAPIGateway.SendGetPlayerInfoRequest` _returnvalue PlayerSub (`|CreateDelegate` :!event `GetPlayerInfoSuccess`) (`|CreateDelegate` :!event `GetPlayerInfoFaulure`)))))

(fn `GetPlayerInfoSuccess`
  (params (PlayerInfomation :type "PlayerInfo Structure"))
  (bind (_playersub _playername _role _customizeitems) (break `PlayerInfo` PlayerInfomation))
  (bind _returnvalue (`AWSSubsystem.GetDynamoDBGateway` (subsystem `AWSSubsystem`)))
  (bind _ps_cloud (`self.GetPlayerStateByPlayerSub` _playersub)
    (:`IsValid`
      (`|ExecutionSequence`
        (:`then_0`
          (`/Game/Platform/System/PlayerState/PS_Cloud.Server_SetUserName` _ps_cloud (`KismetTextLibrary.Conv_StringToText` _playername)))
        (:`then_1`
          (`/Game/Platform/System/PlayerState/PS_Cloud.Server_SetPlayerRoleType` _ps_cloud _role))
        (:`then_2`
          (`self.ServerApplyCustomizeData` _playersub _customizeitems))
        (:`then_3`
          (`/Engine/EditorBlueprintResources/StandardMacros.IsValid` _returnvalue
            (:`Is Valid`
              (bind _returnvalue_2 (`GameplayStatics.GetCurrentLevelName` true))
              (`DynamoDBAPIGateway.SendAddAccessRecordRequest` _returnvalue _playersub _returnvalue_2 (`/Game/Platform/System/BPFL_SystemLib.ConvertDateTimeToString` (`KismetMathLibrary.Now`)) (`|CreateDelegate` :!event `AddAccessRecordSuccess`) (`|CreateDelegate` :!event `AddAccessRecordFailure`)))))
        (:`then_4`)))))

(fn `Initialize Cloud Player`
  (params (`Player Controller` :type "PlayerController Object Reference"))
  (bind _returnvalue (`AWSSubsystem.GetDynamoDBGateway` (subsystem `AWSSubsystem`)))
  (set `self.ServerAssignCharacterEventPlayerController` `Player Controller`)
  (if (`KismetSystemLibrary.IsDedicatedServer`)
    (bind _asps_cloud (cast `/Game/Platform/System/PlayerState/PS_Cloud` (`Controller.PlayerState` `Player Controller`)))
    (bind _playersub (`ProjectTwoPlayerState.PlayerSub` _asps_cloud))
    (if (not (`KismetStringLibrary.IsEmpty` _playersub))
      (`/Engine/EditorBlueprintResources/StandardMacros.IsValid` _returnvalue
        (:`Is Valid`
          (`DynamoDBAPIGateway.SendGetPlayerInfoRequest` _returnvalue _playersub (`|CreateDelegate` :!event `GetPlayerInfoSuccess`) (`|CreateDelegate` :!event `GetPlayerInfoFaulure`)))))))

(fn `IOCPConnectFailure`)

(fn `IOCPConnectSuccess`)

(fn `ServerApplyCustomizeData`
  (params (PlayerSub :type String) (CustomizeData :type "Array of Integer"))
  (bind (_value _returnvalue) (`BlueprintMapLibrary.Map_Find` (`ProjectTwoGameState.PlayerMap` (`/Game/Platform/System/BPFL_SystemLib.GetCloudGameState`)) PlayerSub))
  (if _returnvalue
    (bind _asbp_base_character (cast `/Game/Platform/Character/Base/BP_BaseCharacter` (`Controller.K2_GetPawn` _value)))
    (`CustomizeComponent.SetCustomizeRepData` (`/Game/Platform/Character/Base/BP_BaseCharacter.BP_CustomizeComponent` _asbp_base_character) CustomizeData false)))

(fn `UserConstructionScript`
  (`parent.UserConstructionScript`))