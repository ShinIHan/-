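; GM_Lecture is the lecture game mode that sets up the classroom and spawns participants.
; On BeginPlay it streams the classroom from the GI_Local lecture's data table row, plus an optional personal lab, then after a fixed delay has GameState load the flow data.
; BP_Seat actors are mapped by display name.
; SeatNum only separates admins from players, who spawn above the seat indexed by player count and receive seat references.
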(event `self.ReceiveBeginPlay`
  (bind _gs_base (`/Game/Platform/System/BPFL_SystemLib.GetBaseGameState`))
  (`parent.ReceiveBeginPlay`)
  (bind _asgi_local (cast `/Game/Platform/System/GameInstance/GI_Local` (`/Game/Platform/System/BPFL_SystemLib.GetBaseGameInstance`)))
  (set `self.Lecture` (`/Game/Platform/System/GameInstance/GI_Local.Lecture` _asgi_local))
  (`self.Load_LectureLevel`) ; 여기서 서버에서 지정해준 강의 로드해오면 됨
  (`KismetSystemLibrary.Delay` 2.0) ; 클라이언트 접속 대기
  (set `self.GameStateRef` _gs_base)
  (`/Game/Platform/System/GameState/GS_Base.Load_FlowData` _gs_base (`self.LectureData`)))

(event `self.Server_AssignCharacter`
  (params (Platform :type "/Game/Platform/System/E_Platform Enum" :default "NewEnumerator0") (SeatNum :type Integer) (PlayerController :type "PlayerController Object Reference"))
  (`self.SwitchBySeatNum` SeatNum
    (:`Player`
      (bind _returnvalue (`self.GetNumPlayers`))
      (bind _seat (`self.Get_SeatReference` _returnvalue))
      (bind (_returnvalue_location _returnvalue_rotation _returnvalue_scale) (`KismetMathLibrary.BreakTransform` (`self.GetTransform` _seat)))
      (bind _character (`self.SpawnCharacter` Platform (`KismetMathLibrary.MakeTransform` (+ _returnvalue_location (0.0 0.0 50.0)) _returnvalue_rotation _returnvalue_scale) PlayerController))
      (bind _asbp_base_character (cast `/Game/Platform/Character/Base/BP_BaseCharacter` _character))
      ;[1 1 1] ExpSeats가 비어있지 않으면 실험실 존재
      (set `/Game/Platform/Character/Base/BP_BaseCharacter.Seat Ref` _seat _asbp_base_character)
      (if (`BlueprintMapLibrary.Map_IsNotEmpty` (`self.ExpSeats`))
        (set `/Game/Platform/Character/Base/BP_BaseCharacter.ExpSeat Ref` (`self.Get_ExpSeatReference` _returnvalue) _asbp_base_character)))
    (:`Admin`
      (bind _aspc_local (cast `/Game/Platform/System/PlayerController/PC_Local` PlayerController))
      (`/Game/Platform/System/GameMode/GM_Lobby.SpawnAdminCharacter` (`/Game/Platform/System/BPFL_SystemLib.GetLocalGameMode`) _aspc_local))))

(event `Load_LectureLevel`
  (bind _returnvalue (`|GetDataTableRow` "/Game/Platform/LectureBase/DT_LectureInfoList.DT_LectureInfoList" (`self.Lecture`))
    (:`then`
      (set `self.LectureData` (`.LectureDataTable_15_51AF40DB4FD506C454EC7BB94F18215B` (break `/Game/Platform/Struct/S_LectureInfo` _returnvalue)))
      (`GameplayStatics.LoadStreamLevel` (`self.Get_StreamLevelName` (`.StreamLevel_14_5DFAB8D14C7F6467F97560BDC5D796E9` (break `/Game/Platform/Struct/S_LectureInfo` _returnvalue))) true)
      (bind _outactors (`GameplayStatics.GetAllActorsOfClass` "/Game/Platform/LectureBase/BP_Seat.BP_Seat_C"))
      (for _array_element _outactors
        (`BlueprintMapLibrary.Map_Add` (`self.Seats`) (`KismetSystemLibrary.GetDisplayName` _array_element) _array_element))
      (if (`.PersonalExpLevel_22_DD4B9103442ACEB63B266FAEAEE8A483` (break `/Game/Platform/Struct/S_LectureInfo` _returnvalue))
        ;[1 1 1] 강의가 만약 개인 실험실이 있다면 실험 레벨 스폰 후 Seats와 같은 객체면 강의실 좌석이고 없으면 실험실 좌석
        (`GameplayStatics.LoadStreamLevel` (`self.Get_StreamLevelName` (enumliteral `/Game/Platform/Struct/E_ClassroomType` "NewEnumerator2")) true)
        (bind _outactors_2 (`GameplayStatics.GetAllActorsOfClass` "/Game/Platform/LectureBase/BP_Seat.BP_Seat_C"))
        (for _array_element_2 _outactors_2
          (bind _returnvalue_2 (`KismetSystemLibrary.GetDisplayName` _array_element_2))
          (if (not (`.ReturnValue` (`BlueprintMapLibrary.Map_Find` (`self.Seats`) _returnvalue_2)))
            (`BlueprintMapLibrary.Map_Add` (`self.ExpSeats`) _returnvalue_2 _array_element_2)))))
    (:`RowNotFound`
      (`KismetSystemLibrary.PrintString` "GM_LocalLecture::Load_LectureLevel - Cannot find row name int data table " true true (struct :`R` 1.0 :`A` 1.0) 15.0))))

(fn `Get_ExpSeatReference`
  (params (PlayerIndex :type Integer))
  (returns (Seat :type "/Game/Platform/LectureBase/BP_Seat Object Reference"))
  (bind (_value _returnvalue) (`BlueprintMapLibrary.Map_Find` (`self.ExpSeats`) (`KismetStringLibrary.Concat_StrStr` "BP_Seat" (`KismetStringLibrary.Conv_IntToString` PlayerIndex) "_Exp")))
  (if _returnvalue
    (return _value)
    (else
      (`KismetSystemLibrary.PrintString` "GM_LocalLecture::GetExpSeatReference - Cannot find BP_Seat" true true (struct :`R` 1.0 :`A` 1.0) 20.0)
      (return null))))

(fn `Get_SeatReference`
  (params (PlayerIndex :type Integer))
  (returns (Seat :type "/Game/Platform/LectureBase/BP_Seat Object Reference"))
  (bind (_value _returnvalue) (`BlueprintMapLibrary.Map_Find` (`self.Seats`) (`KismetStringLibrary.Concat_StrStr` "BP_Seat" (`KismetStringLibrary.Conv_IntToString` PlayerIndex))))
  (if _returnvalue
    (return _value)
    (else
      (`KismetSystemLibrary.PrintString` "GM_LocalLecture::GetSeatReference - Cannot find BP_Seat" true true (struct :`R` 1.0 :`A` 1.0) 20.0)
      (return null))))

(fn `Get_StreamLevelName`
  (params (Type :type "/Game/Platform/Struct/E_ClassroomType Enum" :default "NewEnumerator0"))
  (returns (Name :type Name))
  (switch `/Game/Platform/Struct/E_ClassroomType` Type
    (:`NewEnumerator0`
      (return "LV_Classroom_I"))
    (:`NewEnumerator1`
      (return "LV_Classroom_L"))
    (:`NewEnumerator2`
      (return "LV_Classroom_P"))))

(fn `UserConstructionScript`
  (`parent.UserConstructionScript`))