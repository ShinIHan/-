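; Base GameMode that spawns a platform-specific player character (PC or VR) and provides server travel to a named level.
; New players' PC_Base controllers get a client request to assign a character by option, which pairs with Server_AssignCharacter.
; That event spawns the character at a random PlayerStart, possesses it and sets the client's control rotation.
; StartLecture and SkipLecture are empty hooks for child classes, as Local and Cloud modes behave differently.
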(event `self.ReceiveBeginPlay`
  (`parent.ReceiveBeginPlay`))

(event `self.HandleStartingNewPlayer`
  (params (NewPlayer :type "PlayerController Object Reference"))
  ;[1 1 1] Player Spawn
  (bind _aspc_base (cast `/Game/Platform/System/PlayerController/PC_Base` NewPlayer))
  (`/Game/Platform/System/PlayerController/PC_Base.Client_RequestAssignCharacterByOption` _aspc_base))

(event `Server_AssignCharacter`
  (params (Platform :type "/Game/Platform/System/E_Platform Enum" :default "NewEnumerator0") (SeatNum :type Integer) (PlayerController :type "PlayerController Object Reference"))
  (bind (_outitem _outindex) (`KismetArrayLibrary.Array_Random` (`self.GetPlayerStartActors`)))
  ;[1 1 1] Player Spawn
  (if (!= _outindex -1)
    (`self.SpawnCharacter` Platform (`self.GetTransform` _outitem) PlayerController)))

(event `ServerTravel`
  (params (LevelName :type String))
  ;[1 1 1] Server Travel
  (`KismetSystemLibrary.ExecuteConsoleCommand` (`KismetStringLibrary.Concat_StrStr` "servertravel " LevelName) null))

(event `Start Lecture`
  ;[1 1 1] Local과 Cloud의 작동방식의 차이로 상속 구조 이용
)

(event `Skip Lecture`
  ;[1 1 1] Local과 Cloud의 작동방식의 차이로 상속 구조 이용
)

(fn `GetPlayerStartActors`
  (returns (PlayerStartArray :type "Array of PlayerStart Object Reference"))
  (bind _outactors (`GameplayStatics.GetAllActorsOfClass` "/Script/Engine.PlayerStart"))
  (if (> (`KismetArrayLibrary.Array_Length` _outactors) 0)
    (return _outactors)
    (else
      (return))))

(fn `SpawnCharacter`
  (params (Platform :type "/Game/Platform/System/E_Platform Enum" :default "NewEnumerator0") (Transform :type "Transform Structure") (PlayerController :type "PlayerController Object Reference"))
  (returns (Character :type "Character Object Reference"))
  (bind (_transform_location _transform_rotation) (`KismetMathLibrary.BreakTransform` (`local.Transform`)))
  (bind _returnvalue (`|SpawnActorFromClass` (select `/Game/Platform/System/E_Platform` Platform :`NewEnumerator0` (`self.PCCharacter`) :`NewEnumerator1` (`self.VRCharacter`) :!type "Actor Class Reference") Transform "AdjustIfPossibleButAlwaysSpawn" "MultiplyWithRoot" PlayerController null))
  (bind _asbp_base_character (cast `/Game/Platform/Character/Base/BP_BaseCharacter` _returnvalue))
  (`Controller.Possess` PlayerController _asbp_base_character)
  (bind _aspc_base (cast `/Game/Platform/System/PlayerController/PC_Base` PlayerController))
  (`/Game/Platform/System/PlayerController/PC_Base.Client_SetControlRotation` _aspc_base _transform_rotation)
  (return _asbp_base_character))

(fn `UserConstructionScript`)