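; Lobby game mode that spawns a character for each joining player controller according to platform and seat number.
; ServerAssignCharacter uses the SwitchBySeatNum macro to route seat numbers of zero or above to SpawnCharacter and negative ones to the admin path.
; The admin path casts to PC_Local, spawns BP_AdminCharacter and possesses it.
; Both paths spawn at a random player start and do nothing when none exists.
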(event `self.Server_AssignCharacter`
  (params (Platform :type "/Game/Platform/System/E_Platform Enum" :default "NewEnumerator0") (SeatNum :type Integer) (PlayerController :type "PlayerController Object Reference"))
  (bind (_outitem _outindex) (`KismetArrayLibrary.Array_Random` (`self.GetPlayerStartActors`)))
  ;[1 1 1] Character Spawn / Local
  (`self.SwitchBySeatNum` SeatNum
    (:`Player`
      (if (!= _outindex -1)
        (`self.SpawnCharacter` Platform (`self.GetTransform` _outitem) PlayerController)))
    (:`Admin`
      (bind _aspc_local (cast `/Game/Platform/System/PlayerController/PC_Local` PlayerController))
      (`self.SpawnAdminCharacter` _aspc_local))))

(fn `SpawnAdminCharacter`
  (params (PC_Local :type "/Game/Platform/System/PlayerController/PC_Local Object Reference"))
  (bind (_outitem _outindex) (`KismetArrayLibrary.Array_Random` (`self.GetPlayerStartActors`)))
  (if (!= _outindex -1)
    (bind _returnvalue (`|SpawnActorFromClass` "/Game/Platform/Character/Local/BP_AdminCharacter.BP_AdminCharacter_C" (`self.GetTransform` _outitem) "Undefined" "MultiplyWithRoot" null null))
    (`Controller.Possess` PC_Local _returnvalue)))

(fn `UserConstructionScript`
  (`parent.UserConstructionScript`))