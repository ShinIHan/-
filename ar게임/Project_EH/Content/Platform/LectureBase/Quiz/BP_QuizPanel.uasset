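; BP_QuizPanel is a lecture quiz actor that shows timed questions through a WBP_QuizPanel widget.
; BeginPlay loads QuizData table rows into an array, binds widget events for particles and next quiz, then shows the first question with the timer stopped.
; Each NextQuiz initializes the widget, restarts a timeline countdown and advances the index, flagging QuizEnd after the last question.
; Only remote instances update time text and request the next quiz on timeout.
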(event `self.ReceiveBeginPlay`
  (bind _aswbp_quiz_panel (cast `/Game/Platform/LectureBase/Quiz/WBP_QuizPanel` (`WidgetComponent.GetWidget` (`self.Widget`))))
  (set `self.QuizRef` _aswbp_quiz_panel)
  (`|ExecutionSequence`
    (:`then_0`
      (bind _outrownames (`DataTableFunctionLibrary.GetDataTableRowNames` (`self.QuizData`)))
      (for _array_element _outrownames
        (bind _returnvalue (`|GetDataTableRow` (`self.QuizData`) _array_element)
          (:`then`
            (`KismetArrayLibrary.Array_Add` (`self.QuizDataArray`) _returnvalue)))))
    (:`then_1`
      (add `/Game/Platform/LectureBase/Quiz/WBP_QuizPanel.SpawnParticle` (`self.QuizRef`) (delegate `SpawnParticle`))
      (add `/Game/Platform/LectureBase/Quiz/WBP_QuizPanel.NextQuiz` (`self.QuizRef`) (delegate `NextQuiz`))
      (`self.NextQuiz`)
      (`TimelineComponent.Stop` (`self.TimeOutAndNextQuiz`)) ; Sequnce Event를 통한 Timeline Play 필요
    )))

(event `SpawnParticle`
  (`ActorComponent.Activate` (`self.Niagara`) true))

(event `NextQuiz`
  (`/Game/Platform/LectureBase/Quiz/WBP_QuizPanel.Init` (`self.QuizRef`) (`self.QuizEnd`) (`|GetArrayItem` (`self.QuizDataArray`) (`self.CurrIndex`)))
  (`|ExecutionSequence`
    (:`then_0`
      (`self.CalcTimeOut`)
      (if (`self.QuizEnd`)
        (`TimelineComponent.Stop` (`self.TimeOutAndNextQuiz`))))
    (:`then_1`
      (if (< (+ (`self.CurrIndex`) 1) (`KismetArrayLibrary.Array_Length` (`self.QuizDataArray`)))
        (set `self.CurrIndex` (+ (`self.CurrIndex`) 1))
        (else
          ;[1 1 1] 끝
          (set `self.QuizEnd` true))))))

(event `CalcTimeOut`
  (bind (_direction _time) (`Timeline|TimeOutAndNextQuiz` :!via `PlayFromStart`)
    (:`Update`
      (`/Engine/EditorBlueprintResources/ActorMacros.Switch Has Authority`
        (:`Remote`
          (`/Game/Platform/LectureBase/Quiz/WBP_QuizPanel_Question.SetTimeText` (`/Game/Platform/LectureBase/Quiz/WBP_QuizPanel.Question` (`self.QuizRef`)) (`KismetMathLibrary.Round64` _time)))))
    (:`Finished`
      (`/Engine/EditorBlueprintResources/ActorMacros.Switch Has Authority`
        (:`Remote`
          (`/Game/Platform/LectureBase/Quiz/WBP_QuizPanel.CallNextQuiz` (`self.QuizRef`)))))))

(fn `UserConstructionScript`)