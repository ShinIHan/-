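; BP_WhaleMK2 is a whale actor with a skeletal mesh, an animated talking mouth and optional random coloring.
; On BeginPlay it passes MovementAmount to its ABP_WhaleMK2 anim instance.
; Tick watches for changes to Talking, then either plays the Talk timeline to step the Mouth material's Type parameter or stops it and resets Type.
; The construction script can set body and bottom material colors through RandomColor.
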(event `self.ReceiveBeginPlay`
  (`parent.ReceiveBeginPlay`)
  (bind _asabp_whale_mk2 (cast `/Game/Platform/LectureBase/Whale/ABP_WhaleMK2` (`SkeletalMeshComponent.GetAnimInstance` (`self.SkeletalMesh`))))
  (set `/Game/Platform/LectureBase/Whale/ABP_WhaleMK2.MovementAmount` (`self.MovementAmount`) _asabp_whale_mk2))

(event `self.ReceiveTick`
  (params (DeltaSeconds :type "Float (single-precision)"))
  (`parent.ReceiveTick` DeltaSeconds)
  (if (!= (`self.PrevTalking`) (`self.Talking`))
    (`self.Update_MouthType`)
    (set `self.PrevTalking` (`self.Talking`))))

(event `Update_MouthType`
  (if (`self.Talking`)
    (bind (_direction _mouthtype_o) (`Timeline|Talk` :!label _label)
      (:`Update`
        (`MeshComponent.SetScalarParameterValueOnMaterials` (`self.Mouth`) "Type" (`KismetMathLibrary.Conv_IntToDouble` (`KismetMathLibrary.FFloor` _mouthtype_o)))))
    (else
      (`|ExecutionSequence`
        (:`then_0`
          (goto _label :!via `Stop`))
        (:`then_1`
          (`MeshComponent.SetScalarParameterValueOnMaterials` (`self.Mouth`) "Type" 0.0))))))

(fn `UserConstructionScript`
  (bind (_bodycolor _bottomcolor) (`self.RandomColor`))
  (if (`self.UseRandomColor`)
    (`MeshComponent.SetVectorParameterValueOnMaterials` (`self.SkeletalMesh`) "BodyColor" (`KismetMathLibrary.Conv_LinearColorToVector` _bodycolor))
    (`MeshComponent.SetVectorParameterValueOnMaterials` (`self.SkeletalMesh`) "BottomColor" (`KismetMathLibrary.Conv_LinearColorToVector` _bottomcolor))))