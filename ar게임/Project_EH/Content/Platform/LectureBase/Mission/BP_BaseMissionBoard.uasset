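; BP_BaseMissionBoard is a mission board Blueprint that shows missions through a WBP_MissionBoard user widget hosted by its Widget component.
; AddMission passes a Script to the widget, first removing the oldest ToDoList entry when Clear is set and the list holds more than two children.
; CompleteMission forwards completion to the same widget, which owns the display logic.
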(event `Add Mission`
  (params (Script :type String))
  (bind _aswbp_mission_board (cast `/Game/Platform/LectureBase/Mission/WBP_MissionBoard` (`WidgetComponent.GetWidget` (`self.Widget`))))
  (if (`self.Clear`)
    (bind _todolist (`/Game/Platform/LectureBase/Mission/WBP_MissionBoard.ToDoList` _aswbp_mission_board))
    (if (> (`PanelWidget.GetChildrenCount` _todolist) 2)
      (`PanelWidget.RemoveChildAt` _todolist 0)))
  (`/Game/Platform/LectureBase/Mission/WBP_MissionBoard.Add Mission` _aswbp_mission_board Script))

(event `Complete Mission`
  (bind _aswbp_mission_board (cast `/Game/Platform/LectureBase/Mission/WBP_MissionBoard` (`WidgetComponent.GetWidget` (`self.Widget`))))
  (`/Game/Platform/LectureBase/Mission/WBP_MissionBoard.Complete Mission` _aswbp_mission_board))

(fn `UserConstructionScript`)