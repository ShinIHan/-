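; Level actor that plays lecture, quiz or practice sequences and relays mission updates to a MissionBoard.
; It binds to game-state dispatchers at BeginPlay for lectures, or when a locally controlled character overlaps CharacterCheck in practice.
; Dispatched events set and play sequences, change speed, toggle pause and add or complete missions.
; When a sequence finishes, it calls ProcessFlow on the server for lectures and on the remote client for practice.
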(event `self.ReceiveBeginPlay`
  (bind _gs_base (`/Game/Platform/System/BPFL_SystemLib.GetBaseGameState`))
  (`PrimitiveComponent.SetCollisionEnabled` (`self.CharacterCheck`) "NoCollision")
  (if (`self.ForLecture`)
    (add `/Game/Platform/System/GameState/GS_Base.Dispatch_PlaySequence` _gs_base (delegate `PlaySequence`) :!label _label)
    (add `/Game/Platform/System/GameState/GS_Base.Dispatch_SequenceSpeed` _gs_base (delegate `ChangeSpeed`))
    (add `/Game/Platform/System/GameState/GS_Base.Dispatch_SequencePausePlay` _gs_base (delegate `PausePlay`))
    (add `/Game/Platform/System/GameState/GS_Base.Dispatch_Mission` _gs_base (delegate `AddMission`))
    (add `/Game/Platform/System/GameState/GS_Base.Dispatch_MissionComplete` _gs_base (delegate `MissionComplete`))
    (else
      (`PrimitiveComponent.SetCollisionEnabled` (`self.CharacterCheck`) "QueryAndPhysics"))))

(event `self.CharacterCheck.OnComponentBeginOverlap`
  (params (OverlappedComponent :type "PrimitiveComponent Object Reference") (OtherActor :type "Actor Object Reference") (OtherComp :type "PrimitiveComponent Object Reference") (OtherBodyIndex :type Integer) (bFromSweep :type Boolean) (SweepResult :type "HitResult Structure (by ref)"))
  (bind `_as캐릭터` (cast `Character` OtherActor))
  (if (`Pawn.IsLocallyControlled` `_as캐릭터`)
    (goto _label)))

(event `PlaySequence`
  (params (Param :type "/Game/Platform/Struct/S_Flow_PlaySequence Structure"))
  (bind _sequenceplayer (`self.SequencePlayer`))
  (`self.SetSequence` Param_Sequence_2_5E0F85BD4FCCFFB4F4A8939BC9E6357A)
  (add `MovieSceneSequencePlayer.OnFinished` _sequenceplayer (delegate `CompleteSequence`))
  (`MovieSceneSequencePlayer.Play` _sequenceplayer))

(event `CompleteSequence`
  (clear `MovieSceneSequencePlayer.OnFinished` (`self.SequencePlayer`))
  (if true
    (if (`self.ForLecture`)
      (`/Engine/EditorBlueprintResources/ActorMacros.Switch Has Authority` ; 강의와 퀴즈(강의)의 경우 서버에서 Process Flow 호출
        (:`Authority`
          _))
      (else
        (`/Engine/EditorBlueprintResources/ActorMacros.Switch Has Authority` ; 실습의 경우 Remote에서 본인이 Process Flow 실행
          (:`Remote`
            _))))
    (`/Game/Platform/System/GameState/GS_Base.ProcessFlow` (`/Game/Platform/System/BPFL_SystemLib.GetBaseGameState`))))

(event `ChangeSpeed`
  (params (`New Speed` :type "Float (double-precision)"))
  (`MovieSceneSequencePlayer.SetPlayRate` (`self.SequencePlayer`) `New Speed`))

(event `PausePlay`
  (`/Engine/EditorBlueprintResources/StandardMacros.FlipFlop`
    (:`A`
      (`MovieSceneSequencePlayer.Pause` (`self.SequencePlayer`)))
    (:`B`
      (`MovieSceneSequencePlayer.Play` (`self.SequencePlayer`)))))

(event `AddMission`
  (params (Script :type String))
  (bind _missionboard (`self.MissionBoard`))
  (`/Engine/EditorBlueprintResources/StandardMacros.IsValid` _missionboard
    (:`Is Valid`
      (`/Game/Platform/LectureBase/Mission/BP_BaseMissionBoard.Add Mission` _missionboard Script))
    (:`Is Not Valid`
      (`KismetSystemLibrary.PrintString` "BP_LectureSequencePlayer::AddMission - Invalid Mission Board" true true (struct :`R` 1.0 :`A` 1.0) 20.0))))

(event `MissionComplete`
  (bind _missionboard (`self.MissionBoard`))
  (`/Engine/EditorBlueprintResources/StandardMacros.IsValid` _missionboard
    (:`Is Valid`
      (`/Game/Platform/LectureBase/Mission/BP_BaseMissionBoard.Complete Mission` _missionboard))
    (:`Is Not Valid`
      (`KismetSystemLibrary.PrintString` "BP_LectureSequencePlayer::CompleteMission - Invalid Mission Board" true true (struct :`R` 1.0 :`A` 1.0) 20.0))))

(fn `UserConstructionScript`)