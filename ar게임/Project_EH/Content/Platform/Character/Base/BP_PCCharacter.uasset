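; BP_PCCharacter is the desktop (PC) player character, handling Enhanced Input movement, mouse look and grabbing through a Grip component.
; BeginPlay adds the PC and chorded-key mapping contexts on the Remote authority branch only.
; Opened widgets are tracked in an array that blocks game input until empty, and a cursor toggle switches input modes.
; Aim, camera, IK and VR getters return default values, while desired velocity returns normalized horizontal velocity.
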(event `self.ReceiveBeginPlay`
  (bind _returnvalue (pcsubsystem `EnhancedInputLocalPlayerSubsystem` (`/Game/Platform/System/BPFL_SystemLib.GetBasePlayerController`)))
  (`parent.ReceiveBeginPlay`)
  (`/Engine/EditorBlueprintResources/ActorMacros.Switch Has Authority`
    (:`Remote`
      (`EnhancedInputSubsystemInterface.AddMappingContext` _returnvalue "/Game/Platform/Input/IMC_PC.IMC_PC" 1 (struct))
      (`EnhancedInputSubsystemInterface.AddMappingContext` _returnvalue "/Game/Platform/Input/IMC_ChordedKeyInput.IMC_ChordedKeyInput" 0 (struct)))))

(event `self.Open Widget`
  (params (Widget :type "UserWidget Object Reference"))
  ;[0.4989 0.6383 1] 위젯을 배열에 저장 후 게임 입력 차단
  (`UserWidget.AddToViewport` Widget 0)
  (`KismetArrayLibrary.Array_AddUnique` (`self.Widgets`) Widget)
  (`Widget.SetUserFocus` Widget (`/Game/Platform/System/BPFL_SystemLib.GetBasePlayerController`))
  (`self.IgnoreGameInput`))

(event `self.Close Widget by Ref`
  (params (Widget :type "UserWidget Object Reference"))
  (bind _returnvalue (`KismetArrayLibrary.Array_Find` (`self.Widgets`) Widget))
  ;[1 0.4686 0.4786] 위젯을 배열에서 제거 후 배열이 비어있다면 입력 복구
  (if (!= _returnvalue -1)
    (`KismetArrayLibrary.Array_Remove` (`self.Widgets`) _returnvalue)
    (`Widget.RemoveFromParent` Widget)
    (if (== (`KismetArrayLibrary.Array_Length` (`self.Widgets`)) 0)
      (`self.ResetInput`))))

(event `EnhancedInput|/Game/Platform/Input/InputAction/IA_Move`
  (params (ActionValue :type "Vector2D Structure") (ElapsedSeconds :type "Float (double-precision)") (TriggeredSeconds :type "Float (double-precision)") (InputAction :type "InputAction Object Reference" :default "/Game/Platform/Input/InputAction/IA_Move.IA_Move"))
  (:`Triggered`
    (`self.AddMovementInput` (`self.GetActorForwardVector`) (`KismetMathLibrary.SelectFloat` (* ActionValue_X 0.5) (* ActionValue_X 0.3) (== ActionValue_Y 0.0)))
    (`self.AddMovementInput` (`self.GetActorRightVector`) (`KismetMathLibrary.SelectFloat` (* ActionValue_Y 0.5) (* ActionValue_Y 0.3) (== ActionValue_X 0.0)))))

(event `EnhancedInput|/Game/Platform/Input/InputAction/IA_Look`
  (params (ActionValue :type "Vector2D Structure") (ElapsedSeconds :type "Float (double-precision)") (TriggeredSeconds :type "Float (double-precision)") (InputAction :type "InputAction Object Reference" :default "/Game/Platform/Input/InputAction/IA_Look.IA_Look"))
  (:`Triggered`
    (`self.AddControllerYawInput` ActionValue_X)
    (`self.AddControllerPitchInput` ActionValue_Y)))

(event `EnhancedInput|/Game/Platform/Input/InputAction/IA_ToggleMouseCursor`
  (params (ActionValue :type Boolean) (ElapsedSeconds :type "Float (double-precision)") (TriggeredSeconds :type "Float (double-precision)") (InputAction :type "InputAction Object Reference" :default "/Game/Platform/Input/InputAction/IA_ToggleMouseCursor.IA_ToggleMouseCursor"))
  (:`Started`
    (bind _isa (`/Engine/EditorBlueprintResources/StandardMacros.FlipFlop`)
      (:`A`
        _)
      (:`B`
        _))
    (`self.SetInputMode` _isa)))

(event `EnhancedInput|/Game/Platform/Input/InputAction/IA_PC_Grab`
  (params (ActionValue :type Boolean) (ElapsedSeconds :type "Float (double-precision)") (TriggeredSeconds :type "Float (double-precision)") (InputAction :type "InputAction Object Reference" :default "/Game/Platform/Input/InputAction/IA_PC_Grab.IA_PC_Grab"))
  (bind _grip (`self.Grip`))
  (:`Started`
    (`GripComponent.Grip` _grip))
  (:`Completed`
    (`GripComponent.TryDrop` _grip)))

(fn `GetAimValue`
  (returns (Yaw :type "Float (double-precision)") (Pitch :type "Float (double-precision)"))
  (return 0.0 0.0))

(fn `GetCameraLocation`
  (returns (CamLocation :type "Vector Structure"))
  (return (0.0 0.0 0.0)))

(fn `GetDesiredVelocity`
  (returns (Velocity :type "Vector Structure"))
  (bind (_returnvalue_x _returnvalue_y) (`KismetMathLibrary.BreakVector` (`self.GetVelocity`)))
  (return (`KismetMathLibrary.Normal` (`KismetMathLibrary.MakeVector` _returnvalue_x _returnvalue_y))))

(fn `GetUpperBodyIKData`
  (returns (UpperBodyIKData :type "UpperBodyIKData Structure"))
  (return))

(fn `GetVRInitialize`
  (returns (bInitalized :type Boolean))
  (return false))

(fn `SetInputMode`
  (params (bGameInput :type Boolean))
  (bind _pc_base (`/Game/Platform/System/BPFL_SystemLib.GetBasePlayerController`))
  (if bGameInput
    (set `PlayerController.bShowMouseCursor` false _pc_base)
    (`WidgetBlueprintLibrary.SetInputMode_GameOnly` _pc_base)
    (`Controller.ResetIgnoreInputFlags` _pc_base)
    (else
      (set `PlayerController.bShowMouseCursor` true _pc_base)
      (`WidgetBlueprintLibrary.SetInputMode_GameAndUIEx` _pc_base null)
      (`Controller.SetIgnoreLookInput` _pc_base true)
      (`Controller.SetIgnoreMoveInput` _pc_base true))))

(fn `UserConstructionScript`
  (`parent.UserConstructionScript`))