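; Text chat component for a character that shows messages in a chat bubble and a text chat log.
; A server event relays player name and text to a multicast event, which updates both displays only on non-server instances, so a listen-server host is skipped.
; The bubble is the component's own widget, while the log widget is lazily fetched from the base character and cached.
; Empty player names appear as "Unknown" in the log.
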(event `Multi_TextChatEvent`
  (params (PlayerName :type String) (Str :type String))
  (if (not (or (`KismetSystemLibrary.IsServer`) (`KismetSystemLibrary.IsDedicatedServer`)))
    (`self.AddChatBubbleText` Str)
    (`self.AddTextToTextChat` (`KismetStringLibrary.Concat_StrStr` (`KismetMathLibrary.SelectString` PlayerName "Unknown " (`KismetStringLibrary.NotEqual_StrStr` PlayerName)) " : " Str))))

(event `Server_TextChatEvent`
  (params (PlayerName :type String) (Str :type String))
  (`self.Multi_TextChatEvent` PlayerName Str))

(fn `AddChatBubbleText`
  (params (Str :type String))
  (bind _aswbp_chat_bubble (cast `/Game/Widget/Chat/WBP_ChatBubble` (`self.GetWidget`)))
  (`/Game/Widget/Chat/WBP_ChatBubble.UpdateChat` _aswbp_chat_bubble Str))

(fn `AddTextToTextChat`
  (params (Str :type String))
  (`/Game/Widget/Chat/WBP_TextChatWidget.AddChat` (`self.GetTextChatWidget`) Str))

(fn `GetTextChatWidget`
  (returns (TextChat :type "/Game/Widget/Chat/WBP_TextChatWidget Object Reference"))
  (bind _textchatwidget (`/Game/Platform/Character/Base/BP_BaseCharacter.TextChatWidget` (`/Game/Platform/System/BPFL_SystemLib.GetBaseCharacter`)))
  (`/Engine/EditorBlueprintResources/StandardMacros.IsValid` (`self.TextChatWidget`)
    (:`Is Valid`
      _)
    (:`Is Not Valid`
      (`/Engine/EditorBlueprintResources/StandardMacros.IsValid` _textchatwidget
        (:`Is Valid`
          (set `self.TextChatWidget` _textchatwidget)))))
  (return (`self.TextChatWidget`)))