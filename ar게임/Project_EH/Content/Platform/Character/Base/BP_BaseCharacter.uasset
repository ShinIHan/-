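; Base player character for PC and VR, providing subtitles, overhead name tags, input-lock helpers and a lecture management debug widget toggle.
; A SwitchNetworkByLocation macro limits startup and subtitle display to standalone or the owning client.
; Subtitles auto-hide through a timeline sized by text length, and name tags are set only for Cloud game instances, hidden from their owner.
; Widget open/close and default gadget setup are empty hooks.
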(event `self.ReceiveBeginPlay`
  (`self.SwitchNetworkByLocation`
    (:`Standalone`
      _)
    (:`MyClient`
      _))
  (`self.Initialize`)
  (`/Game/Platform/System/PlayerController/PC_Base.CameraFadeIn` (`/Game/Platform/System/BPFL_SystemLib.GetBasePlayerController`) 1.0)
  (`PrimitiveComponent.SetOnlyOwnerSee` (`self.HeadLessCharacterMesh`) true))

(event `Initialize`
  (`Controller.SetControlRotation` (`GameplayStatics.GetPlayerController` 0) (`self.K2_GetActorRotation`))
  (`self.Initialize_DefaultWidget`)
  (`self.Initialize_DefaultGadget`)
  (`self.SetUserNameByType`) ; Game Instance의 Type을 통한 UserName Set
)

(event `self.ReceiveTick`
  (params (DeltaSeconds :type "Float (single-precision)"))
  (`parent.ReceiveTick` DeltaSeconds))

(event `Open Widget`
  (params (Widget :type "UserWidget Object Reference")))

(event `Close Widget by Ref`
  (params (Widget :type "UserWidget Object Reference")))

(event `Initialize_DefaultWidget`
  ;[1 0.1354 0.1354] Debug
  (bind _returnvalue (`|CreateWidget` "/Game/Widget/Subtitle/WBP_Subtitle.WBP_Subtitle_C"))
  (bind _output_get (set `self.Subtitle` _returnvalue))
  (`UserWidget.AddToViewport` _output_get 0)
  (`self.ShowSubtitle` "자막 예시 공간"))

(event `ShowSubtitle`
  (params (Script :type String))
  ;[1 1 1] Subtitle
  (`self.SwitchNetworkByLocation`
    (:`Standalone`
      _)
    (:`MyClient`
      _))
  (`/Game/Widget/Subtitle/WBP_Subtitle.ShowSubtitle` (`self.Subtitle`) Script)
  (`TimelineComponent.SetTimelineLength` (`self.ShowSubitleTimeLine`) (`self.CalculateExpressionTimeBySubtitleLength` Script))
  (`Timeline|ShowSubitleTimeLine` :!via `PlayFromStart` ; 새로운 자막이 들어올때마다 0에서부터 시작
    (:`Finished`
      (`self.HideSubtitle`))))

(event `HideSubtitle`
  ;[1 1 1] Subtitle
  (`/Game/Widget/Subtitle/WBP_Subtitle.HideSubtitle` (`self.Subtitle`)))

(event `EnhancedInput|/Game/Platform/Input/InputAction/IA_OpenDebugWidget`
  (params (ActionValue :type Boolean) (ElapsedSeconds :type "Float (double-precision)") (TriggeredSeconds :type "Float (double-precision)") (InputAction :type "InputAction Object Reference" :default "/Game/Platform/Input/InputAction/IA_OpenDebugWidget.IA_OpenDebugWidget"))
  (bind _lecture_management_widget (`/Game/Platform/System/PlayerController/PC_Base.Lecture Management Widget` (`/Game/Platform/System/BPFL_SystemLib.GetBasePlayerController`)))
  ;[1 0.1771 0.1771] Open Debug Widget / PC, VR 모두 사용
  (:`Started`
    (`/Engine/EditorBlueprintResources/StandardMacros.FlipFlop`
      (:`A`
        (`self.Open Widget` _lecture_management_widget))
      (:`B`
        (`self.Close Widget by Ref` _lecture_management_widget)))))

(event `Initialize_DefaultGadget`)

(fn `CalculateExpressionTimeBySubtitleLength`
  (params (Script :type String))
  (returns (ReturnValue :type "Float (double-precision)"))
  (return (+ (* (`KismetStringLibrary.Len` Script) (`self.TimePerLetter`)) (`self.TimeOffset`))))

(fn `IgnoreGameInput`
  (bind `_as플레이어_컨트롤러` (cast `PlayerController` (`self.GetController`)))
  (set `PlayerController.bShowMouseCursor` true `_as플레이어_컨트롤러`)
  (`Controller.SetIgnoreMoveInput` `_as플레이어_컨트롤러` true)
  (`Controller.SetIgnoreLookInput` `_as플레이어_컨트롤러` true))

(fn `ResetInput`
  (bind `_as플레이어_컨트롤러` (cast `PlayerController` (`self.GetController`)))
  (`WidgetBlueprintLibrary.SetInputMode_GameOnly` `_as플레이어_컨트롤러`)
  (set `PlayerController.bShowMouseCursor` false `_as플레이어_컨트롤러`)
  (`Controller.ResetIgnoreLookInput` `_as플레이어_컨트롤러`)
  (`Controller.ResetIgnoreInputFlags` `_as플레이어_컨트롤러`))

(fn `SetSubtitleLocation`
  (bind _output_get (set `self.SubtitleLocation` (cast `/Game/Widget/Subtitle/E_SubtitleLocation` (+ (`self.SubtitleLocation`) 1))))
  (if (> (`KismetMathLibrary.Conv_ByteToInt` _output_get) 2)
    (set `self.SubtitleLocation` "NewEnumerator0"))
  (`/Game/Widget/Subtitle/WBP_Subtitle.SetSubtitleLocation` (`self.Subtitle`) (`self.SubtitleLocation`)))

(fn `SetUserName`
  (params (RecvUserName :type Text))
  (set `self.UserName` RecvUserName)
  (`TextRenderComponent.K2_SetText` (`self.FrontUserName`) (`self.UserName`))
  (`TextRenderComponent.K2_SetText` (`self.BackUserName`) (`self.UserName`)))

(fn `SetUserNameByType`
  (if (`|EnumEquality` (`ProjectTwoGameInstance.Type` (`/Game/Platform/System/BPFL_SystemLib.GetBaseGameInstance`)) "TE_Cloud")
    (`self.SetUserName` (`self.UserName`)) ; Cloud의 경우에만 User Name Set을 진행
    (`PrimitiveComponent.SetOwnerNoSee` (`self.FrontUserName`) true)
    (`PrimitiveComponent.SetOwnerNoSee` (`self.BackUserName`) true) ; 본인 캐릭터 머리위의 닉네임은 보이지 않도록 수정
    (else
      (`SceneComponent.SetVisibility` (`self.UserNamePosComponent`) false true))))

(fn `UserConstructionScript`)