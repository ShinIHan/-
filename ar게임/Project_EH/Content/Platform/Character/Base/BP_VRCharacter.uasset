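; VR player character that drives body IK from headset and motion controllers, with switchable walk or teleport/snap-turn locomotion.
; Initialization aligns tracking origin to the mesh eye socket and multicasts the height offset.
; Local ticks feed IK effectors, hand auto-posing and a smoothed camera-yaw-following subtitle.
; Spawned teleporter and per-hand widget pointers join grip input, world-space widget panels and a level-gated fingertip pointer.
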(event `self.ReceiveBeginPlay`
  (`parent.ReceiveBeginPlay`)
  (set `self.Movement Mode` "NewEnumerator0"))

(event `self.Initialize`
  (`parent.Initialize`)
  (`self.VRIKInitialize`)
  (`self.SwitchNetworkByLocation`
    (:`Standalone`
      _)
    (:`MyClient`
      _))
  (`EnhancedInputSubsystemInterface.AddMappingContext` (pcsubsystem `EnhancedInputLocalPlayerSubsystem` (`/Game/Platform/System/BPFL_SystemLib.GetBasePlayerController`)) "/Game/Platform/Input/IMC_VR.IMC_VR" 0 (struct)))

(event `VRIKInitialize`
  (`HeadMountedDisplayFunctionLibrary.EnableHMD` true)
  (`HeadMountedDisplayFunctionLibrary.SetTrackingOrigin` "Floor")
  (`VRInverseKinematicsComponent.InitialzieBoneLenghtToSkeletalMesh` (`self.VRInverseKinematics`) (`self.Mesh`))
  (`self.SetVRTransform`)
  (`PrimitiveComponent.SetOwnerNoSee` (`self.Mesh`) true)
  (`PrimitiveComponent.SetRenderInMainPass` (`self.HeadLessCharacterMesh`) false)
  (`self.VRHandInitialize`) ; Hand Init
)

(event `SetVRTransform`
  (bind _output_get (set `self.VRInitalized` true))
  (`self.Server_VRIKInitialize` _output_get (`self.CalcVROffset`)))

(event `self.ReceiveTick`
  (params (DeltaSeconds :type "Float (single-precision)"))
  (bind (_capsulecomponent _camera _leftmotioncontroller _rightmotioncontroller) (`self.GetEffectorsWorldTransform`))
  (`parent.ReceiveTick` DeltaSeconds)
  (`self.SwitchNetworkByLocation`
    (:`Standalone`
      _)
    (:`MyClient`
      _))
  (`VRInverseKinematicsComponent.SetEffectorTransforms` (`self.VRInverseKinematics`) _capsulecomponent _camera _leftmotioncontroller _rightmotioncontroller) ; IK Update
  (`|ExecutionSequence`
    (:`then_0`
      (if (`self.IsValidChildActors`)
        ;[1 1 1] Hand & Finger Widget Interaction
        (`/Game/Platform/VRSystem/Hand/BP_VRHand_AutoPosing.TrackingInput` (`self.LeftHandChildActor`) (`|GetInputActionValue`) (`|GetInputActionValue`) (`|GetInputActionValue`))
        (if (`self.IsFingerWidgetActive`)
          (`/Game/Platform/VRSystem/Hand/BP_VRHand_AutoPosing.TrackingInput` (`self.RIghtHandChildActor`) (`|GetInputActionValue`) (`|GetInputActionValue`) (`|GetInputActionValue`))
          (`self.FingerTrackingToRightHandPosition` (`self.FingerWidgetInteraction`) (`self.RIghtHandChildActor`))
          (else
            (`/Game/Platform/VRSystem/Hand/BP_VRHand_AutoPosing.TrackingInput` (`self.RIghtHandChildActor`) (`|GetInputActionValue`) (`|GetInputActionValue`) (`|GetInputActionValue`))))))
    (:`then_1`
      (`self.UpdateSubtitleRotation` DeltaSeconds) ; Subtitle
    )))

(event `self.Initialize_DefaultGadget`
  (`parent.Initialize_DefaultGadget`) ; Base Character 에서 생성되는 가젯이 있다면 필요
  (`|ExecutionSequence`
    (:`then_0`
      (`self.SpawnTeleportor`))
    (:`then_1`
      (`self.SpawnWidgetInteractionActorsOnBothHands`))
    (:`then_2`
      (`self.SpawnFingerWidgetInteractionActorOnRightHand`))))

(event `self.Initialize_DefaultWidget`
  ;[1 1 1] Default Widget
  (`parent.Initialize_DefaultWidget`) ; WBP Subtitle 생성
  (`WidgetComponent.SetWidget` (`self.SubtitileLocationComponent`) (`self.Subtitle`)) ; Subtitle Widget Component에 부모에서 생성된 WBP Subtitle을 Set
)

(event `self.Open Widget`
  (params (Widget :type "UserWidget Object Reference"))
  ;[1 1 1] Open Widget / Close Widget
  (`/Engine/EditorBlueprintResources/StandardMacros.IsValid` Widget
    (:`Is Valid`
      (bind _location (`self.SetVRWidgetActorSpawnTransformLocation` (`self.RepCamera`) (`self.WidgetDistance`) (`self.WidgetOffset`)))
      (bind _returnvalue (`|SpawnActorFromClass` "/Game/Platform/VRSystem/InterativeWidget/BP_AttachedWidget.BP_AttachedWidget_C" (`KismetMathLibrary.MakeTransform` _location (struct :`Yaw` 180.0) (0.2 0.2 0.2)) "AlwaysSpawn" "MultiplyWithRoot" null Widget null))
      (`BlueprintMapLibrary.Map_Add` (`self.OpenWidgetActors`) Widget _returnvalue))))

(event `self.Close Widget by Ref`
  (params (Widget :type "UserWidget Object Reference"))
  (bind (_value _returnvalue) (`BlueprintMapLibrary.Map_Find` (`self.OpenWidgetActors`) Widget))
  ;[1 1 1] Open Widget / Close Widget
  (if _returnvalue
    (`/Engine/EditorBlueprintResources/StandardMacros.IsValid` _value
      (:`Is Valid`
        (`self.K2_DestroyActor` _value)
        (`BlueprintMapLibrary.Map_Remove` (`self.OpenWidgetActors`) Widget)))))

(event `EnhancedInput|/Game/Platform/Input/InputAction/IA_Move`
  (params (ActionValue :type "Vector2D Structure") (ElapsedSeconds :type "Float (double-precision)") (TriggeredSeconds :type "Float (double-precision)") (InputAction :type "InputAction Object Reference" :default "/Game/Platform/Input/InputAction/IA_Move.IA_Move"))
  (bind (_returnvalue_location _returnvalue_rotation) (`KismetMathLibrary.BreakTransform` (`SceneComponent.K2_GetComponentToWorld` (`self.RepCamera`))))
  (bind (_returnvalue_location_2 _returnvalue_rotation_2) (`KismetMathLibrary.BreakTransform` (`SceneComponent.K2_GetComponentToWorld` (`self.RepCamera`))))
  ;[1 1 1 0.9] Movement
  ;;[1 1 1] Walking
  (:`Triggered`
    (switch `/Game/Platform/Struct/E_VRMovement` (`self.Movement Mode`)
      (:`NewEnumerator0`
        (`self.AddMovementInput` (`KismetMathLibrary.GetForwardVector` _returnvalue_rotation) ActionValue_X)
        (`self.AddMovementInput` (`KismetMathLibrary.GetRightVector` _returnvalue_rotation_2) ActionValue_Y)))))

(event `EnhancedInput|/Game/Platform/Input/InputAction/IA_VR_Rotate`
  (params (ActionValue :type "Float (double-precision)") (ElapsedSeconds :type "Float (double-precision)") (TriggeredSeconds :type "Float (double-precision)") (InputAction :type "InputAction Object Reference" :default "/Game/Platform/Input/InputAction/IA_VR_Rotate.IA_VR_Rotate"))
  ;[1 1 1 0.9] Movement
  ;;[1 1 1] Teleport
  (:`Triggered`
    (switch `/Game/Platform/Struct/E_VRMovement` (`self.Movement Mode`)
      (:`NewEnumerator1`
        (`self.Input_SnapTurn` ActionValue)))))

(event `EnhancedInput|/Game/Platform/Input/InputAction/IA_VR_SwitchMovement`
  (params (ActionValue :type Boolean) (ElapsedSeconds :type "Float (double-precision)") (TriggeredSeconds :type "Float (double-precision)") (InputAction :type "InputAction Object Reference" :default "/Game/Platform/Input/InputAction/IA_VR_SwitchMovement.IA_VR_SwitchMovement"))
  ;[1 1 1 0.9] Movement
  ;;[1 1 1] Switch VR Movement Mode
  (:`Started`
    (switch `/Game/Platform/Struct/E_VRMovement` (`self.Movement Mode`)
      (:`NewEnumerator0`
        (set `self.Movement Mode` "NewEnumerator1"))
      (:`NewEnumerator1`
        (set `self.Movement Mode` "NewEnumerator0")))))

(event `EnhancedInput|/Game/Platform/Input/InputAction/IA_VR_Teleport`
  (params (ActionValue :type "Float (double-precision)") (ElapsedSeconds :type "Float (double-precision)") (TriggeredSeconds :type "Float (double-precision)") (InputAction :type "InputAction Object Reference" :default "/Game/Platform/Input/InputAction/IA_VR_Teleport.IA_VR_Teleport"))
  ;[1 1 1 0.9] Movement
  ;;[1 1 1] Teleport
  (:`Triggered`
    (switch `/Game/Platform/Struct/E_VRMovement` (`self.Movement Mode`) :!label _label
      (:`NewEnumerator1`
        (`self.Input_TeleportEvent` ActionValue))))
  (:`Completed`
    (goto _label)))

(event `EnhancedInput|/Game/Platform/Input/InputAction/IA_VR_LeftGrab`
  (params (ActionValue :type Boolean) (ElapsedSeconds :type "Float (double-precision)") (TriggeredSeconds :type "Float (double-precision)") (InputAction :type "InputAction Object Reference" :default "/Game/Platform/Input/InputAction/IA_VR_LeftGrab.IA_VR_LeftGrab"))
  (bind _leftgrip (`self.LeftGrip`))
  ;[1 1 1] Grip
  (:`Started`
    (`GripComponent.Grip` _leftgrip))
  (:`Completed`
    (`GripComponent.TryDrop` _leftgrip)))

(event `EnhancedInput|/Game/Platform/Input/InputAction/IA_VR_RightGrab`
  (params (ActionValue :type Boolean) (ElapsedSeconds :type "Float (double-precision)") (TriggeredSeconds :type "Float (double-precision)") (InputAction :type "InputAction Object Reference" :default "/Game/Platform/Input/InputAction/IA_VR_RightGrab.IA_VR_RightGrab"))
  (bind _rightgrip (`self.RightGrip`))
  ;[1 1 1] Grip
  (:`Started`
    (`GripComponent.Grip` _rightgrip))
  (:`Completed`
    (`GripComponent.TryDrop` _rightgrip)))

(event `EnhancedInput|/Game/Platform/Input/InputAction/IA_VR_LeftTrigger`
  (params (ActionValue :type Boolean) (ElapsedSeconds :type "Float (double-precision)") (TriggeredSeconds :type "Float (double-precision)") (InputAction :type "InputAction Object Reference" :default "/Game/Platform/Input/InputAction/IA_VR_LeftTrigger.IA_VR_LeftTrigger"))
  (bind _leftwidgetinteraction (`self.LeftWidgetInteraction`))
  (bind _leftwidgetinteraction_2 (`self.LeftWidgetInteraction`))
  ;[1 1 1] Trigger
  (:`Started`
    (`/Engine/EditorBlueprintResources/StandardMacros.IsValid` _leftwidgetinteraction
      (:`Is Valid`
        (`/Game/Platform/VRSystem/WidgetInteraction/BP_VRWidgetInteraction.ActiveWidgetInteraction` _leftwidgetinteraction_2 true))))
  (:`Completed`
    (`/Engine/EditorBlueprintResources/StandardMacros.IsValid` _leftwidgetinteraction
      (:`Is Valid`
        (`/Game/Platform/VRSystem/WidgetInteraction/BP_VRWidgetInteraction.ActiveWidgetInteraction` _leftwidgetinteraction_2 false)))))

(event `EnhancedInput|/Game/Platform/Input/InputAction/IA_VR_RightTrigger`
  (params (ActionValue :type Boolean) (ElapsedSeconds :type "Float (double-precision)") (TriggeredSeconds :type "Float (double-precision)") (InputAction :type "InputAction Object Reference" :default "/Game/Platform/Input/InputAction/IA_VR_RightTrigger.IA_VR_RightTrigger"))
  (bind _rightwidgetinteraction (`self.RightWidgetInteraction`))
  (bind _rightwidgetinteraction_2 (`self.RightWidgetInteraction`))
  ;[1 1 1] Trigger
  (:`Started`
    (`/Engine/EditorBlueprintResources/StandardMacros.IsValid` _rightwidgetinteraction_2
      (:`Is Valid`
        (`/Game/Platform/VRSystem/WidgetInteraction/BP_VRWidgetInteraction.ActiveWidgetInteraction` _rightwidgetinteraction true))))
  (:`Completed`
    (`/Engine/EditorBlueprintResources/StandardMacros.IsValid` _rightwidgetinteraction_2
      (:`Is Valid`
        (`/Game/Platform/VRSystem/WidgetInteraction/BP_VRWidgetInteraction.ActiveWidgetInteraction` _rightwidgetinteraction false)))))

(event `Server_VRIKInitialize`
  (params (VRInitialized :type Boolean) (Offset :type "Float (double-precision)"))
  (`self.Multi_VRIKInitialize` VRInitialized Offset))

(event `Multi_VRIKInitialize`
  (params (VRInitialized :type Boolean) (Offset :type "Float (double-precision)"))
  (`self.SwitchNetworkByLocation`
    (:`Server`
      _)
    (:`Client`
      _))
  (bind _output_get (set `self.VRInitalized` VRInitialized))
  (set `self.HMDOffset` Offset)
  (if _output_get
    (`SceneComponent.K2_SetRelativeLocation` (`self.VRSystemOriginComponent`) (`KismetMathLibrary.MakeVector` 0.0 0.0 Offset) false false)))

(fn `CalcVROffset`
  (returns (Offset :type "Float (double-precision)"))
  (bind (_returnvalue_x _returnvalue_y _returnvalue_z) (`KismetMathLibrary.BreakVector` (`SceneComponent.K2_GetComponentLocation` (`self.RepCamera`))))
  (bind _output_get (set `self.HMDOffset` (- (.z (.location (`SceneComponent.GetSocketTransform` (`self.Mesh`) "Eye" "RTS_World"))) _returnvalue_z)))
  (return _output_get))

(fn `FingerTrackingToRightHandPosition`
  (params (FingerWidgetInteraction :type "SceneComponent Object Reference") (`Right Hand Child Actor` :type "SkeletalMeshActor Object Reference"))
  (bind _returnvalue (`SceneComponent.GetSocketTransform` (`SkeletalMeshActor.SkeletalMeshComponent` `Right Hand Child Actor`) "index_03_r" "RTS_Component"))
  (`SceneComponent.K2_SetRelativeLocation` FingerWidgetInteraction (.location _returnvalue) false false)
  (`SceneComponent.K2_SetRelativeRotation` FingerWidgetInteraction (`KismetMathLibrary.MakeRotator` 0.0 (.pitch (.rotation _returnvalue)) (.yaw (.rotation _returnvalue))) false false))

(fn `GetAimValue`
  (returns (Yaw :type "Float (double-precision)") (Pitch :type "Float (double-precision)"))
  (return 0.0 0.0))

(fn `GetCameraLocation`
  (returns (CamLocation :type "Vector Structure"))
  (bind _repcamera (`self.RepCamera`))
  (`/Engine/EditorBlueprintResources/StandardMacros.IsValid` _repcamera
    (:`Is Valid`
      (return (`SceneComponent.RelativeLocation` _repcamera)))))

(fn `GetDesiredVelocity`
  (returns (Velocity :type "Vector Structure"))
  (return (0.0 0.0 0.0)))

(fn `GetEffectorsWorldTransform`
  (returns (CapsuleComponent :type "Transform Structure") (Camera :type "Transform Structure") (LeftMotionController :type "Transform Structure") (RightMotionController :type "Transform Structure"))
  (return (`SceneComponent.K2_GetComponentToWorld` (`self.CapsuleComponent`)) (`SceneComponent.K2_GetComponentToWorld` (`self.RepCamera`)) (`SceneComponent.K2_GetComponentToWorld` (`self.LeftRepMotionController`)) (`SceneComponent.K2_GetComponentToWorld` (`self.RightRepMotionController`))))

(fn `GetOriginTransform`
  (returns (OriginTransform :type "Transform Structure"))
  (return (`SceneComponent.K2_GetComponentToWorld` (`self.RepCamera`))))

(fn `GetUpperBodyIKData`
  (returns (UpperBodyIKData :type "UpperBodyIKData Structure"))
  (bind _vrinversekinematics (`self.VRInverseKinematics`))
  (`/Engine/EditorBlueprintResources/StandardMacros.IsValid` _vrinversekinematics
    (:`Is Valid`
      (return (`VRInverseKinematicsComponent.UpperBodyIKData` _vrinversekinematics)))
    (:`Is Not Valid`
      (`KismetSystemLibrary.PrintString` "VRInverse Kinematics is not valid"))))

(fn `GetVRInitialize`
  (returns (bInitalized :type Boolean))
  (return (`self.VRInitalized`)))

(fn `HideSubtitle`
  (`parent.HideSubtitle`)
  (set `self.IsSubtitleActive` false))

(fn `InitFingerWidgetInteractionComponent`
  (params (WidgetInteractionComponent :type "ChildActorComponent Object Reference"))
  (bind _asbp_vrfinger_widget_interaction (cast `/Game/Platform/VRSystem/WidgetInteraction/BP_VRFingerWidgetInteraction` (`ChildActorComponent.ChildActor` WidgetInteractionComponent)))
  (bind _output_get (set `self.Finger wiidget interaction Actor` _asbp_vrfinger_widget_interaction))
  (bind _widgetinteraction (`/Game/Platform/VRSystem/WidgetInteraction/BP_VRFingerWidgetInteraction.WidgetInteraction` _output_get))
  (set `WidgetInteractionComponent.InteractionDistance` 1.5 _widgetinteraction)
  (set `WidgetInteractionComponent.PointerIndex` 2 _widgetinteraction)
  (set `WidgetInteractionComponent.VirtualUserIndex` 2 _widgetinteraction)
  (`/Game/Platform/VRSystem/WidgetInteraction/BP_VRFingerWidgetInteraction.SetFingerWidgetActivation` (`self.Finger wiidget interaction Actor`) true))

(fn `Input_SnapTurn`
  (params (AxisValue :type "Float (double-precision)"))
  (bind _returnvalue (> (`KismetMathLibrary.Abs` (`local.AxisValue`)) (`self.SnapTurnThreshold`)))
  (if (`self.TurnFlag`)
    (if (not _returnvalue)
      (set `self.TurnFlag` false))
    (elif _returnvalue
      (set `self.TurnFlag` true)
      (`Controller.SetControlRotation` (`self.GetController`) (`KismetMathLibrary.ComposeRotators` (`self.GetControlRotation`) (`KismetMathLibrary.MakeRotator` 0.0 0.0 (* (`self.SnapTurnAngle`) (`KismetMathLibrary.SignOfFloat` (`local.AxisValue`)))))))))

(fn `Input_TeleportEvent`
  (params (AxisValue :type "Float (double-precision)"))
  (bind (_origintransform_location _origintransform_rotation) (`KismetMathLibrary.BreakTransform` (`self.GetOriginTransform`)))
  (bind _teleporter (`self.Teleporter`))
  (`/Engine/EditorBlueprintResources/StandardMacros.IsValid` (`self.Teleporter`)
    (:`Is Valid`
      (if (> (`KismetMathLibrary.Abs` AxisValue) (`self.Teleport Input Threshold`))
        (if (> (`local.AxisValue`) 0.0)
          (`/Game/Platform/VRSystem/Teleporter/BP_Teleporter.ActivateTeleporter` (`self.Teleporter`))
          (elif (not (`self.BackStepFlag`))
            (`/Game/Platform/System/PlayerController/PC_Base.Server_Teleport` (`/Game/Platform/System/BPFL_SystemLib.GetBasePlayerController`) (+ (`self.K2_GetActorLocation`) (* (`KismetMathLibrary.GetForwardVector` _origintransform_rotation) (* (`self.BackStepDistance`) 0.0))) (`self.GetControlRotation`))
            (set `self.BackStepFlag` true)))
        (elif (`/Game/Platform/VRSystem/Teleporter/BP_Teleporter.IsActivate` (`self.Teleporter`))
          (if (`/Game/Platform/VRSystem/Teleporter/BP_Teleporter.LastFrameValidDestination` _teleporter)
            (`/Game/Platform/System/PlayerController/PC_Base.Server_Teleport` (`/Game/Platform/System/BPFL_SystemLib.GetBasePlayerController`) (`/Game/Platform/VRSystem/Teleporter/BP_Teleporter.Last Valid Location` _teleporter) (`self.K2_GetActorRotation`)))
          (`/Game/Platform/VRSystem/Teleporter/BP_Teleporter.DisableTeleporter` (`self.Teleporter`))
          (elif (`self.BackStepFlag`)
            (set `self.BackStepFlag` false)))))))

(fn `IsFingerWidgetInteractionActiveLevel`
  (returns (ReturnValue :type Boolean))
  (bind _returnvalue (`GameplayStatics.GetCurrentLevelName` true))
  (return (`KismetStringLibrary.EqualEqual_StrStr` _returnvalue "LV_Sample")))

(fn `IsValidChildActors`
  (returns (ReturnValue :type Boolean))
  (if (`self.IsFingerWidgetActive`)
    (return (and (`KismetSystemLibrary.IsValid` (`self.LeftHandChildActor`)) (`KismetSystemLibrary.IsValid` (`self.RIghtHandChildActor`)) (`KismetSystemLibrary.IsValid` (`self.Finger wiidget interaction Actor`))))
    (else
      (return (and (`KismetSystemLibrary.IsValid` (`self.LeftHandChildActor`)) (`KismetSystemLibrary.IsValid` (`self.RIghtHandChildActor`)))))))

(fn `OnRep_HMDOffset`)

(fn `SetVRWidgetActorSpawnTransformLocation`
  (params (RepCamera :type "RepCameraComponent Object Reference") (WidgetDistance :type "Float (double-precision)") (WidgetOffset :type "Vector Structure"))
  (returns (Location :type "Vector Structure"))
  (bind (_returnvalue_roll _returnvalue_pitch _returnvalue_yaw) (`KismetMathLibrary.BreakRotator` (`SceneComponent.K2_GetComponentRotation` RepCamera)))
  (return (+ (+ (`SceneComponent.K2_GetComponentLocation` RepCamera) (* (`KismetMathLibrary.GetForwardVector` (`KismetMathLibrary.MakeRotator` 0.0 0.0 _returnvalue_yaw)) WidgetDistance)) WidgetOffset)))

(fn `ShowSubtitle`
  (params (Script :type String))
  (`parent.ShowSubtitle` Script)
  (set `self.IsSubtitleActive` true)
  (return))

(fn `SpawnFingerWidgetInteractionActorOnRightHand`
  (bind _returnvalue (`self.IsFingerWidgetInteractionActiveLevel`))
  (if _returnvalue
    (set `self.IsFingerWidgetActive` _returnvalue)
    (`self.InitFingerWidgetInteractionComponent` (`self.FingerWidgetInteraction`))
    (else
      (`ActorComponent.K2_DestroyComponent` (`self.FingerWidgetInteraction`)))))

(fn `SpawnTeleportor`
  (bind _returnvalue (`|SpawnActorFromClass` "/Game/Platform/VRSystem/Teleporter/BP_Teleporter.BP_Teleporter_C" (`self.GetTransform`) "Undefined" "SelectDefaultAtRuntime" self null))
  (bind _output_get (set `self.Teleporter` _returnvalue))
  (`self.K2_AttachToComponent` _output_get (`self.RightAim`) "None" "SnapToTarget" "SnapToTarget" "KeepWorld" true))

(fn `SpawnWidgetInteractionActorsOnBothHands`
  (bind _returnvalue (`|SpawnActorFromClass` "/Game/Platform/VRSystem/WidgetInteraction/BP_VRWidgetInteraction.BP_VRWidgetInteraction_C" (`self.GetTransform`) "Undefined" "SelectDefaultAtRuntime" self null))
  (bind _output_get (set `self.LeftWidgetInteraction` _returnvalue))
  (`self.K2_AttachToComponent` _output_get (`self.LeftAim`) "None" "SnapToTarget" "SnapToTarget" "KeepWorld" true)
  (bind _widgetinteraction (`/Game/Platform/VRSystem/WidgetInteraction/BP_VRWidgetInteraction.WidgetInteraction` _output_get))
  (set `WidgetInteractionComponent.PointerIndex` 0 _widgetinteraction)
  (set `WidgetInteractionComponent.VirtualUserIndex` 0 _widgetinteraction)
  (bind _returnvalue_2 (`|SpawnActorFromClass` "/Game/Platform/VRSystem/WidgetInteraction/BP_VRWidgetInteraction.BP_VRWidgetInteraction_C" (`self.GetTransform`) "Undefined" "SelectDefaultAtRuntime" self null))
  (bind _output_get_2 (set `self.RightWidgetInteraction` _returnvalue_2))
  (`self.K2_AttachToComponent` _output_get_2 (`self.RightAim`) "None" "SnapToTarget" "SnapToTarget" "KeepWorld" true)
  (bind _widgetinteraction_2 (`/Game/Platform/VRSystem/WidgetInteraction/BP_VRWidgetInteraction.WidgetInteraction` _output_get_2))
  (set `WidgetInteractionComponent.PointerIndex` 1 _widgetinteraction_2)
  (set `WidgetInteractionComponent.VirtualUserIndex` 1 _widgetinteraction_2))

(fn `UpdateSubtitleRotation`
  (params (DeltaTime :type "Float (double-precision)"))
  (locals (SubtitleOffset :type "Vector Structure" :default (0.0 0.0 100.0)))
  (bind (_relativerotation_roll _relativerotation_pitch _relativerotation_yaw) (`KismetMathLibrary.BreakRotator` (`SceneComponent.RelativeRotation` (`self.RepCamera`))))
  (if (`self.IsSubtitleActive`)
    (`SceneComponent.K2_SetRelativeTransform` (`self.SubtitileLocationComponent`) (`KismetMathLibrary.TInterpTo` (`SceneComponent.GetRelativeTransform` (`self.SubtitileLocationComponent`)) (`KismetMathLibrary.MakeTransform` (+ (`local.SubtitleOffset`) (* (`KismetMathLibrary.Conv_RotatorToVector` (`KismetMathLibrary.MakeRotator` 0.0 0.0 _relativerotation_yaw)) (`self.SubtitleDistance`))) (`KismetMathLibrary.MakeRotator` 0.0 0.0 (+ _relativerotation_yaw 180.0)) (0.1 0.1 0.1)) (`local.DeltaTime`) (`self.SubtitleRotationSpeed`)) false false)))

(fn `UserConstructionScript`
  (`parent.UserConstructionScript`))

(fn `VRHandInitialize`
  (`|ExecutionSequence`
    (:`then_0`
      (bind _asbp_vrhand_auto_posing_left (cast `/Game/Platform/VRSystem/Hand/BP_VRHand_AutoPosing_Left` (`ChildActorComponent.ChildActor` (`self.LeftHand`)))
        (:`then`
          (set `self.LeftHandChildActor` _asbp_vrhand_auto_posing_left)
          (bind _asbp_vrhand_auto_posing (cast `/Game/Platform/VRSystem/Hand/BP_VRHand_AutoPosing` (`ChildActorComponent.ChildActor` (`self.RightHand`)))
            (:`then`
              (set `self.RIghtHandChildActor` _asbp_vrhand_auto_posing))
            (:`CastFailed`
              (`KismetSystemLibrary.PrintString` "Right Cast Failed"))))
        (:`CastFailed`
          (`KismetSystemLibrary.PrintString` "Left Cast Failed"))))
    (:`then_1`
      (`SceneComponent.SetVisibility` (`Actor.RootComponent` (`ChildActorComponent.ChildActor` (`self.RightHand`))) true false)
      (`SceneComponent.SetVisibility` (`Actor.RootComponent` (`ChildActorComponent.ChildActor` (`self.LeftHand`))) true false)
      (`SceneComponent.SetVisibility` (`self.RightHand`) true false)
      (`SceneComponent.SetVisibility` (`self.LeftHand`) true false))))