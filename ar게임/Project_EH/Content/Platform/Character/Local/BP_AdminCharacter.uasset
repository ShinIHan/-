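; Admin player character for a lecture platform, with first-person style movement, look and a lecture management UI.
; On remote BeginPlay it adds the PC input mapping and shows the lecture management widget.
; SetCameraView switches the view target to a given camera and frees the cursor.
; A cursor toggle flips SetInputMode between game-only control and game-and-UI with move and look ignored; diagonal movement is scaled down.
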(event `self.ReceiveBeginPlay`
  (`/Engine/EditorBlueprintResources/ActorMacros.Switch Has Authority`
    (:`Remote`
      (`EnhancedInputSubsystemInterface.AddMappingContext` (pcsubsystem `EnhancedInputLocalPlayerSubsystem` (`GameplayStatics.GetPlayerController` 0)) "/Game/Platform/Input/IMC_PC.IMC_PC" 0 (struct))
      (bind _returnvalue (`|CreateWidget` "/Game/Widget/LectureManagement/WBP_LectureManagement.WBP_LectureManagement_C" null false true))
      (bind _output_get (set `self.LectureManagerWidget` _returnvalue))
      (`UserWidget.AddToViewport` _output_get 0))))

(event `SetCameraView`
  (params (Cam :type "CameraActor Object Reference"))
  (set `self.IsCamActivate` true)
  (set `self.LastCam` Cam)
  (`PlayerController.SetViewTargetWithBlend` (`/Game/Platform/System/BPFL_SystemLib.GetBasePlayerController`) Cam 0.0 "VTBlend_Linear" 0.0 false)
  (`self.SetInputMode` false))

(event `EnhancedInput|/Game/Platform/Input/InputAction/IA_Move`
  (params (ActionValue :type "Vector2D Structure") (ElapsedSeconds :type "Float (double-precision)") (TriggeredSeconds :type "Float (double-precision)") (InputAction :type "InputAction Object Reference" :default "/Game/Platform/Input/InputAction/IA_Move.IA_Move"))
  (:`Triggered`
    (`self.AddMovementInput` (`self.GetActorForwardVector` (`self.GetController`)) (`KismetMathLibrary.SelectFloat` (* ActionValue_X 0.5) (* ActionValue_X 0.3) (== ActionValue_Y 0.0)))
    (`self.AddMovementInput` (`self.GetActorRightVector` (`self.GetController`)) (`KismetMathLibrary.SelectFloat` (* ActionValue_Y 0.5) (* ActionValue_Y 0.3) (== ActionValue_X 0.0)))))

(event `EnhancedInput|/Game/Platform/Input/InputAction/IA_Look`
  (params (ActionValue :type "Vector2D Structure") (ElapsedSeconds :type "Float (double-precision)") (TriggeredSeconds :type "Float (double-precision)") (InputAction :type "InputAction Object Reference" :default "/Game/Platform/Input/InputAction/IA_Look.IA_Look"))
  (:`Triggered`
    (`self.AddControllerYawInput` ActionValue_X)
    (`self.AddControllerPitchInput` ActionValue_Y)))

(event `EnhancedInput|/Game/Platform/Input/InputAction/IA_ToggleMouseCursor`
  (params (ActionValue :type Boolean) (ElapsedSeconds :type "Float (double-precision)") (TriggeredSeconds :type "Float (double-precision)") (InputAction :type "InputAction Object Reference" :default "/Game/Platform/Input/InputAction/IA_ToggleMouseCursor.IA_ToggleMouseCursor"))
  (:`Started`
    (bind _isa (`/Engine/EditorBlueprintResources/StandardMacros.FlipFlop`)
      (:`A`
        _)
      (:`B`
        _))
    (`self.SetInputMode` _isa)))

(fn `SetInputMode`
  (params (bGameInput :type Boolean))
  (bind _pc_base (`/Game/Platform/System/BPFL_SystemLib.GetBasePlayerController`))
  (if bGameInput
    (set `PlayerController.bShowMouseCursor` false _pc_base)
    (`WidgetBlueprintLibrary.SetInputMode_GameOnly` _pc_base)
    (`Controller.ResetIgnoreInputFlags` _pc_base)
    (else
      (set `PlayerController.bShowMouseCursor` true _pc_base)
      (`WidgetBlueprintLibrary.SetInputMode_GameAndUIEx` _pc_base null)
      (`Controller.SetIgnoreLookInput` _pc_base true)
      (`Controller.SetIgnoreMoveInput` _pc_base true))))

(fn `UserConstructionScript`)