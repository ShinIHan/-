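; BP_LocalPCCharacter is a local PC character Blueprint that gives itself a random appearance when play begins.
; On BeginPlay it calls SetRandomCustomize, which reseeds a random stream and sets the customize component's character type to Clay.
; It builds a list of item IDs, one fixed and the rest drawn from per-category ranges, writes it to the component's rep data and applies the items.
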(event `self.ReceiveBeginPlay`
  (`parent.ReceiveBeginPlay`)
  (`self.SetRandomCustomize`))

(fn `SetRandomCustomize`
  (bind _randomstream (`self.RandomStream`))
  (bind _bp_customizecomponent (`self.BP_CustomizeComponent`))
  (bind _customizedata (`self.CustomizeData`))
  (`KismetMathLibrary.SetRandomStreamSeed` (`self.RandomStream`) (`KismetMathLibrary.RandomInteger` 999))
  (`CustomizeComponent.SetCharacterType` _bp_customizecomponent "Clay")
  (`KismetArrayLibrary.Array_Add` _customizedata 1001)
  (`KismetArrayLibrary.Array_Add` _customizedata (`KismetMathLibrary.RandomIntegerInRangeFromStream` _randomstream 2001 2025))
  (`KismetArrayLibrary.Array_Add` _customizedata (`KismetMathLibrary.RandomIntegerInRangeFromStream` _randomstream 3001 3005))
  (`KismetArrayLibrary.Array_Add` _customizedata (`KismetMathLibrary.RandomIntegerInRangeFromStream` _randomstream 4001 4007))
  (`KismetArrayLibrary.Array_Add` _customizedata (`KismetMathLibrary.RandomIntegerInRangeFromStream` _randomstream 5001 5005))
  (set `CustomizeComponent.CustomizeRepData` (make `CustomizeRepData` "Clay" _customizedata) _bp_customizecomponent)
  (`CustomizeComponent.ApplyCustomizeRepItems` (`self.BP_CustomizeComponent`)))

(fn `UserConstructionScript`
  (`parent.UserConstructionScript`))